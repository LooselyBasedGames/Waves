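; BPItemSpawnTarget is a spawn point that creates an item of a configurable class at its own transform.
; It spawns one item on BeginPlay and assigns itself as that item's Parent.
; When a BP_PickupCube stops overlapping its Box, a timer calls Spawn again after SpawnFrequency, replenishing the point.
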(event OnComponentEndOverlap(Box)
  (params (OverlappedComponent :type Primitive%20Component%20Object%20Reference) (OtherActor :type Actor%20Object%20Reference) (OtherComp :type Primitive%20Component%20Object%20Reference) (OtherBodyIndex :type Integer))
  (Utilities|Casting|CastToBP_PickupCube OtherActor)
  (Utilities|Time|SetTimerbyFunctionName 0 "Spawn" (Variables|Default|GetSpawnFrequency)))

(event EventBeginPlay
  (CallFunction|Spawn))

(fn ConstructionScript)

(fn Spawn
  (bind _returnvalue (Game|SpawnActorfromClass (Variables|Default|GetItemToSpawn) (Transformation|GetActorTransform) "Undefined" 0 0))
  (Variables|/Game/VirtualRealityBP/Blueprints/BP_PickupCube.BP_PickupCube_C|SetParent _returnvalue self))