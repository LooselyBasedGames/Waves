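; Player controller that creates the screen indicator HUD and an example UI widget, and tracks which pawn the player is aiming at.
; On BeginPlay it adds both widgets to the viewport.
; Every tick it line-traces from the camera along its forward vector for Pawn objects, ignoring the controlled pawn, and passes the hit actor, or null, to the screen indicator as its focused agent.
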(event EventBeginPlay
  (Utilities|FlowControl|Sequence
    (:then_0
      (bind _returnvalue (UserInterface|CreateWidget "/Game/ScreenIndicator/SICore/ScreenIndicator.ScreenIndicator_C"))
      (bind _output_get (Variables|Default|SetScreenIndicator _returnvalue))
      (UserInterface|Viewport|AddtoViewport _output_get 0))
    (:then_1
      (bind _returnvalue_2 (UserInterface|CreateWidget "/Game/ScreenIndicator/UI/UI_Example.UI_Example_C"))
      (UserInterface|Viewport|AddtoViewport _returnvalue_2 0))))

(event EventTick
  (params (DeltaSeconds :type Float%20%28single-precision%29))
  (bind _playercameramanager (Variables|Default|GetPlayerCameraManager))
  (bind _returnvalue (Camera|GetCameraLocation _playercameramanager))
  ;[1 1 1] Find focused screen indicator agent
  (Utilities|FlowControl|Sequence
    (:then_0
      (bind (_outhit _returnvalue_2) (Collision|LineTraceForObjects _returnvalue (+ _returnvalue (* (Math|Vector|GetForwardVector (Camera|GetCameraRotation _playercameramanager)) 1e+04)) (Utilities|Array|MakeArray "ObjectTypeQuery3") false (Utilities|Array|MakeArray (Pawn|GetControlledPawn)) "None"))
      (if _returnvalue_2
        ;;[1 1 1] Found.
        (Default|SetFocusAgentActor (Variables|Default|GetScreenIndicator) (.HitActor (Collision|BreakHitResult _outhit)))
        (else
          ;;[1 1 1] Not Found. Call with NULL object
          (Default|SetFocusAgentActor (Variables|Default|GetScreenIndicator)))))))

(fn ConstructionScript)