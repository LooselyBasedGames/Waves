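; Base enemy character for a wave game that moves to targets, attacks them and adds its score value to the game mode on death.
; AI MoveTo results and target-destroyed events set the enemy controller's state.
; A looping timer damages both the player pawn and current move target until the associated attack target is destroyed.
; Empty fall/get-up events and mesh-based capsule reset helpers support standing up again.
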(event Custom|MoveToTarget
  (params (TargetToMoveTo :type Actor%20Object%20Reference) (AcceptanceRadius :type Float%20%28single-precision%29))
  (bind _enemycontroller (Variables|Default|GetEnemyController))
  (Game|BindEventtoOnDestroyed TargetToMoveTo (delegate Custom|OnTargetDestroyed))
  (AI|AIMoveTo self "0, 0, 0" TargetToMoveTo AcceptanceRadius false
    (:OnSuccess
      (Default|SetState (Variables|Default|GetEnemyController) "NewEnumerator1"))
    (:OnFail
      (Variables|/Game/Blueprints/LastStandBlueprints/Enemies/BP_BaseEnemyController.BP_BaseEnemyController_C|SetCurrentTarget _enemycontroller 0)
      (Default|SetState _enemycontroller "NewEnumerator0"))))

(event Custom|Attack
  (bind _asbp_base_player_pawn (Utilities|Casting|CastToBP_BasePlayerPawn (Game|Player|GetPlayerPawn 0))
    (:then
      (Default|TakeDamage _asbp_base_player_pawn (Variables|Default|GetDamage)))
    (:CastFailed
      _))
  (bind _asbp_move_target (Utilities|Casting|CastToBP_MoveTarget (Variables|/Game/Blueprints/LastStandBlueprints/Enemies/BP_BaseEnemyController.BP_BaseEnemyController_C|GetCurrentTarget (Variables|Default|GetEnemyController))))
  (Utilities|IsValid _asbp_move_target
    (:Is%20Valid
      (Default|TakeDamage _asbp_move_target (Variables|Default|GetDamage)))))

(event Custom|OnTargetDestroyed
  (params (DestroyedActor :type Actor%20Object%20Reference))
  (bind _enemycontroller (Variables|Default|GetEnemyController))
  (Variables|/Game/Blueprints/LastStandBlueprints/Enemies/BP_BaseEnemyController.BP_BaseEnemyController_C|SetCurrentTarget _enemycontroller 0)
  (Default|SetState _enemycontroller "NewEnumerator0"))

(event Custom|BeginAttack
  (params (MoveTarget :type BP%20Move%20Target%20Object%20Reference))
  (bind _associatedattacktarget (Variables|/Game/Blueprints/LastStandBlueprints/Environment/BP_MoveTarget.BP_MoveTarget_C|GetAssociatedAttackTarget MoveTarget))
  (Utilities|IsValid MoveTarget
    (:Is%20Valid
      (Utilities|IsValid _associatedattacktarget
        (:Is%20Valid
          (Game|BindEventtoOnDestroyed _associatedattacktarget (delegate Custom|StopAttacking))
          (Utilities|Time|SetTimerbyFunctionName 0 "Attack" (Variables|Default|GetAttackFrequency) true))))))

(event Custom|StopAttacking
  (params (DestroyedActor :type Actor%20Object%20Reference))
  (bind _enemycontroller (Variables|Default|GetEnemyController))
  (Utilities|Time|ClearTimerbyFunctionName 0 "Attack")
  (Variables|/Game/Blueprints/LastStandBlueprints/Enemies/BP_BaseEnemyController.BP_BaseEnemyController_C|SetCurrentTarget _enemycontroller 0)
  (Default|SetState _enemycontroller "NewEnumerator0"))

(event Custom|StartFalling)

(event Custom|Die
  (bind _asbp_base_waves_game_mode (Utilities|Casting|CastToBP_BaseWavesGameMode (Game|GetGameMode)))
  (Variables|/Game/Blueprints/LastStandBlueprints/GameModes/BP_BaseWavesGameMode.BP_BaseWavesGameMode_C|SetScore _asbp_base_waves_game_mode (+ (Variables|/Game/Blueprints/LastStandBlueprints/GameModes/BP_BaseWavesGameMode.BP_BaseWavesGameMode_C|GetScore _asbp_base_waves_game_mode) (Variables|Default|GetScoreValue))))

(event Custom|GetUp)

(event Custom|StopMoving
  (bind _enemycontroller (Variables|Default|GetEnemyController))
  (Utilities|IsValid _enemycontroller
    (:Is%20Valid
      (AI|Navigation|StopMovement _enemycontroller))))

(event EventBeginPlay
  (bind _asbp_base_enemy_controller (Utilities|Casting|CastToBP_BaseEnemyController (Pawn|GetController)))
  (Variables|Default|SetEnemyController _asbp_base_enemy_controller))

(fn ConstructionScript)

(fn GetStandUpLocation
  (bind _mesh (Variables|Character|GetMesh))
  (bind _returnvalue (Transformation|GetWorldLocation _mesh))
  (bind _output_get (LocalVariables|SetStandUpLocation (Math|Vector|MakeVector (.x _returnvalue) (.y _returnvalue) (Variables|/Script/Engine.CapsuleComponent|GetCapsuleHalfHeight (Variables|Collision|GetCapsuleComponent)))))
  (return _output_get))

(fn GetStandUpRotation
  (return (Math|Rotator|FindLookatRotation (Variables|/Script/Engine.SceneComponent|GetRelativeLocation (Variables|Character|GetMesh)) (Transformation|GetActorLocation (Variables|/Game/Blueprints/LastStandBlueprints/Enemies/BP_BaseEnemyController.BP_BaseEnemyController_C|GetCurrentTarget (Variables|Default|GetEnemyController))))))

(fn ResetCharacter
  (Transformation|SetActorLocationAndRotation (CallFunction|GetStandUpLocation) "0, 0, 0")
  (Transformation|AttachComponentToComponent (Variables|Character|GetMesh) (Variables|Collision|GetCapsuleComponent) "None" "SnapToTarget" "SnapToTarget" "SnapToTarget" true)
  (Transformation|SetRelativeLocationAndRotation (Variables|Character|GetMesh) (Math|Vector|MakeVector 0.0 0.0 (* (Variables|/Script/Engine.CapsuleComponent|GetCapsuleHalfHeight (Variables|Collision|GetCapsuleComponent)) -1.0)) "0.000000,-90.000000,0.000000" false true))