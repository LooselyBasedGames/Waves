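; BP_LittleEnemy is the little robot enemy, a child Blueprint that extends the behavior of its parent enemy class.
; Dying and starting to fall call the parent, then turn on mesh physics simulation.
; Getting up calls the parent, resets the character, turns simulation off and sets a state on the enemy controller.
; Attack events and the construction script only forward to the parent.
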(event EventStopAttacking
  (params (DestroyedActor :type Actor%20Object%20Reference))
  (|CallParentFunction DestroyedActor))

(event EventDie
  (|CallParentFunction)
  (Physics|SetSimulatePhysics (Variables|Character|GetMesh) true))

(event EventStartFalling
  (|CallParentFunction)
  (Physics|SetSimulatePhysics (Variables|Character|GetMesh) true))

(event EventAttack
  (|CallParentFunction))

(event EventGetUp
  (|CallParentFunction)
  (CallFunction|ResetCharacter)
  (Physics|SetSimulatePhysics (Variables|Character|GetMesh) false)
  (Default|SetState (Variables|Default|GetEnemyController) "NewEnumerator0"))

(event EventBeginAttack
  (params (MoveTarget :type BP%20Move%20Target%20Object%20Reference))
  (|CallParentFunction MoveTarget))

(fn ConstructionScript
  (|CallParentFunction))