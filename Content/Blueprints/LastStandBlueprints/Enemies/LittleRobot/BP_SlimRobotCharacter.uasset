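; Slim robot enemy character that walks to a random BP_MoveTarget and attacks it, extending parent enemy events.
; It picks another target when movement fails or the current one is invalid; FindNewTarget rebuilds the target list, undoing any prior filtering.
; A hit ragdolls the mesh with an impulse-driven force and calls Die.
; StandUp ends physics, snaps capsule and mesh back together, and resumes targeting.
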(event EventTargetDestroyed
  (|CallParentFunction)
  (CallFunction|StopAttacking))

(event EventDie
  (|CallParentFunction))

(event EventMoveFailed
  (|CallParentFunction)
  (bind _newtarget (CallFunction|FindNewTarget))
  (CallFunction|MovetoTarget _newtarget))

(event EventTick
  (params (DeltaSeconds :type Float%20%28single-precision%29))
  (Utilities|IsValid (Variables|Default|GetCurrentTarget)
    (:Is%20Not%20Valid
      (CallFunction|FilterOutCurrentTarget)
      (bind _newtarget (CallFunction|FindNewTarget))
      (CallFunction|MovetoTarget _newtarget))))

(event EventBeginFalling
  (params (FallDuration :type Float%20%28single-precision%29))
  (|CallParentFunction FallDuration)
  (Physics|SetSimulatePhysics (Variables|Character|GetMesh) true))

(event EventTargetReached
  (|CallParentFunction)
  (CallFunction|BeginAttacking 1.0))

(event EventStandUp
  (|CallParentFunction)
  (Physics|SetSimulatePhysics (Variables|Character|GetMesh) false)
  (CallFunction|OrientCharacter)
  (CallFunction|FilterOutCurrentTarget)
  (bind _newtarget (CallFunction|FindNewTarget))
  (CallFunction|MovetoTarget _newtarget))

(event EventAbsorbHit
  (params (HitImpulse :type Vector) (HitBone :type Name))
  (|CallParentFunction HitImpulse HitBone)
  (CallFunction|BeginFalling 5.0)
  (Physics|AddForce (Variables|Character|GetMesh) HitImpulse HitBone false)
  (CallFunction|Die))

(event EventAttack
  (bind _currenttarget (Variables|Default|GetCurrentTarget))
  (|CallParentFunction)
  (Utilities|IsValid _currenttarget
    (:Is%20Valid
      (Default|TakeDamage _currenttarget (Variables|Default|GetAttackDamage)))))

(event EventInit
  (bind _outactors (Actor|GetAllActorsOfClass "/Game/Blueprints/LastStandBlueprints/Environment/BP_MoveTarget.BP_MoveTarget_C"))
  (Variables|Default|SetAllTargets _outactors)
  (bind _newtarget (CallFunction|FindNewTarget))
  (CallFunction|MovetoTarget _newtarget))

(fn ConstructionScript
  (|CallParentFunction))

(fn OrientCharacter
  (bind _mesh (Variables|Character|GetMesh))
  (bind _returnvalue (Transformation|GetWorldLocation _mesh))
  (Transformation|SetActorLocation (Math|Vector|MakeVector (.x _returnvalue) (.y _returnvalue) (+ (.z _returnvalue) (Variables|/Script/Engine.CapsuleComponent|GetCapsuleHalfHeight (Variables|Default|GetCapsuleComponent)))) false false)
  (Transformation|AttachComponentToComponent (Variables|Character|GetMesh) (Variables|Default|GetCapsuleComponent) "None" "SnapToTarget" "SnapToTarget" "SnapToTarget" false)
  (Transformation|SetRelativeLocationAndRotation (Variables|Character|GetMesh) "0, 0,-90.000000" "0,-90.000000, 0" false false))

(fn FindNewTarget
  (bind _outactors (Actor|GetAllActorsOfClass "/Game/Blueprints/LastStandBlueprints/Environment/BP_MoveTarget.BP_MoveTarget_C"))
  (Variables|Default|SetAllTargets _outactors)
  (bind _randomactor (CallFunction|GetRandomItem (Variables|Default|GetAllTargets)))
  (bind _asbp_move_target (Utilities|Casting|CastToBP_MoveTarget _randomactor)
    (:then
      (return _asbp_move_target))
    (:CastFailed
      (return 0))))

(fn GetRandomItem
  (params (List :type Array%20of%20Actor%20Object%20References))
  (return (Utilities|Array|Get(acopy) List (Math|Random|RandomIntegerinRange 0 (- (Utilities|Array|Length List) 1)))))

(fn FilterOutCurrentTarget
  (for (_array_element _array_index) (Variables|Default|GetAllTargets)
    (if (== _array_element (Variables|Default|GetCurrentTarget))
      (Utilities|Array|RemoveIndex (Variables|Default|GetAllTargets) _array_index))))