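; Base enemy character for the wave-based game mode, which attacks the target linked to its AI controller's current move target.
; Attacks turn the enemy to face that target, then deal damage through the BP_TakeDamage interface.
; FallDown ragdolls the mesh for a stun period, after which StandUp moves the actor to the mesh and reattaches it.
; Die leaves a permanent ragdoll, releases the controller, increments the game mode score and destroys the actor after a delay.
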(event Custom|AttackTarget
  (params (TargetToAttack :type Actor%20Object%20Reference))
  (if (Utilities|DoesObjectImplementInterface TargetToAttack "/Game/Blueprints/LastStandBlueprints/Interfaces/BP_TakeDamage.BP_TakeDamage_C")
    (Class|BPTakeDamage|TakeDamage(Message) TargetToAttack (Variables|Default|GetAttackDamage))))

(event Custom|FaceAttackTarget
  (bind _asbp_base_aicontroller (Utilities|Casting|CastToBP_BaseAIController (Pawn|GetController)))
  (bind _asbp_move_target (Utilities|Casting|CastToBP_MoveTarget (Variables|/Game/Blueprints/LastStandBlueprints/Enemies/Controllers/BP_BaseAIController.BP_BaseAIController_C|GetCurrentTarget _asbp_base_aicontroller)))
  (Utilities|IsValid (Variables|/Game/Blueprints/LastStandBlueprints/Environment/BP_MoveTarget.BP_MoveTarget_C|GetAssociatedAttackTarget _asbp_move_target)
    (:Is%20Valid
      (CallFunction|FaceLocation (Math|Vector|MakeVector (.x (Transformation|GetActorLocation (Variables|/Game/Blueprints/LastStandBlueprints/Environment/BP_MoveTarget.BP_MoveTarget_C|GetAssociatedAttackTarget _asbp_move_target))) (.y (Transformation|GetActorLocation (Variables|/Game/Blueprints/LastStandBlueprints/Environment/BP_MoveTarget.BP_MoveTarget_C|GetAssociatedAttackTarget _asbp_move_target))) (.z (Transformation|GetActorLocation)))))))

(event Custom|OnDeath
  (Actor|DestroyActor))

(event Custom|TryToAttack
  (bind _targettoattack (CallFunction|GetTargettoAttack))
  (CallFunction|FaceAttackTarget)
  (Utilities|IsValid _targettoattack
    (:Is%20Valid
      (CallFunction|AttackTarget _targettoattack))))

(event Custom|FallDown
  (params (DownTime :type Float%20%28single-precision%29))
  (if (not (Variables|Default|GetisDead))
    (Variables|Default|SetisStunned true)
    (Physics|SetSimulatePhysics (Variables|Character|GetMesh) true)
    (Utilities|Time|SetTimerbyFunctionName 0 "StandUp" DownTime)))

(event Custom|Die
  (bind _returnvalue (Pawn|GetController))
  (Utilities|Time|ClearTimerbyFunctionName 0 "StandUp")
  (if (not (Variables|Default|GetisDead))
    (Utilities|IsValid _returnvalue
      (:Is%20Valid
        (AI|Navigation|StopMovement _returnvalue)
        (Pawn|UnPossess _returnvalue)
        (Variables|Default|SetisDead true)
        (Variables|Default|SetisStunned true)
        (Variables|Default|SetisAttacking false)
        (Physics|SetSimulatePhysics (Variables|Character|GetMesh) true)
        (Components|DestroyComponent (Variables|Collision|GetCapsuleComponent))
        (Utilities|Time|SetTimerbyEvent (delegate Custom|OnDeath) 1e+01)
        (bind _asbp_base_waves_game_mode (Utilities|Casting|CastToBP_BaseWavesGameMode (Game|GetGameMode)))
        (Math|Integer|IncrementInt (Variables|/Game/Blueprints/LastStandBlueprints/GameModes/BP_BaseWavesGameMode.BP_BaseWavesGameMode_C|GetScore _asbp_base_waves_game_mode))))))

(event Custom|FaceLocation
  (params (AttackTargetLocation :type Vector))
  (Transformation|SetActorRotation (Math|Rotator|FindLookatRotation (Transformation|GetActorLocation) AttackTargetLocation)))

(event Custom|StandUp
  (bind _mesh (Variables|Character|GetMesh))
  (bind _returnvalue (Transformation|GetWorldLocation _mesh))
  (Physics|SetSimulatePhysics (Variables|Character|GetMesh) false)
  (Transformation|SetActorLocation (Math|Vector|MakeVector (.x _returnvalue) (.y _returnvalue) (+ (.z _returnvalue) (Variables|/Script/Engine.CapsuleComponent|GetCapsuleHalfHeight (Variables|Collision|GetCapsuleComponent)))) false false)
  (CallFunction|FaceAttackTarget)
  (Transformation|AttachComponentToComponent (Variables|Character|GetMesh) (Variables|Collision|GetCapsuleComponent) "None" "SnapToTarget" "SnapToTarget" "SnapToTarget" true)
  (Transformation|SetRelativeLocationAndRotation (Variables|Character|GetMesh) (Math|Vector|MakeVector 0.0 0.0 (* (Variables|/Script/Engine.CapsuleComponent|GetCapsuleHalfHeight (Variables|Collision|GetCapsuleComponent)) -1.0)) "0,-90.000000, 0" false false)
  (Variables|Default|SetisStunned false))

(fn ConstructionScript)

(fn GetTargettoAttack
  (bind _asbp_base_aicontroller (Utilities|Casting|CastToBP_BaseAIController (Pawn|GetController))
    (:then
      (bind _asbp_move_target (Utilities|Casting|CastToBP_MoveTarget (Variables|/Game/Blueprints/LastStandBlueprints/Enemies/Controllers/BP_BaseAIController.BP_BaseAIController_C|GetCurrentTarget _asbp_base_aicontroller))
        (:then
          (return (Variables|/Game/Blueprints/LastStandBlueprints/Environment/BP_MoveTarget.BP_MoveTarget_C|GetAssociatedAttackTarget _asbp_move_target)))
        (:CastFailed
          (return 0))))
    (:CastFailed
      (return 0))))

(fn GetAttackTargetLocation
  (bind _asbp_base_aicontroller (Utilities|Casting|CastToBP_BaseAIController (Pawn|GetController))
    (:then
      (bind _asbp_move_target (Utilities|Casting|CastToBP_MoveTarget (Variables|/Game/Blueprints/LastStandBlueprints/Enemies/Controllers/BP_BaseAIController.BP_BaseAIController_C|GetCurrentTarget _asbp_base_aicontroller))
        (:then
          (return (Transformation|GetActorLocation (Variables|/Game/Blueprints/LastStandBlueprints/Environment/BP_MoveTarget.BP_MoveTarget_C|GetAssociatedAttackTarget _asbp_move_target))))
        (:CastFailed
          (return "0, 0, 0"))))
    (:CastFailed
      (return "0, 0, 0"))))