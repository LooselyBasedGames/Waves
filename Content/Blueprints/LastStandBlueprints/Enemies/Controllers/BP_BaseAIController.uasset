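; Base AI controller for attacking enemies, running the BT_EnemyAttacker behavior tree on the BB_EnemyAttacker blackboard.
; On BeginPlay it picks a random TargetPoint in the level as the blackboard attack target and starts the tree.
; Init repeats that setup but stores the random pick only in CurrentTarget, without writing it to the blackboard.
; SetNewTarget accepts only TargetPoints, updating both CurrentTarget and the blackboard key.
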(event Custom|Init
  (bind _blackboardcomponent (Class|AIController|UseBlackboard "/Game/Blueprints/LastStandBlueprints/Enemies/Controllers/BB_EnemyAttacker.BB_EnemyAttacker"))
  (Variables|Default|SetCurrentBlackboard _blackboardcomponent)
  (bind _outactors (Actor|GetAllActorsOfClass "/Script/Engine.TargetPoint"))
  (Variables|Default|SetCurrentTarget (Utilities|Array|Get(acopy) _outactors (Math|Random|RandomIntegerinRange 0 (- (Utilities|Array|Length _outactors) 1))))
  (AI|RunBehaviorTree "/Game/Blueprints/LastStandBlueprints/Enemies/Controllers/BT_EnemyAttacker.BT_EnemyAttacker"))

(event Custom|SetNewTarget
  (params (NewTarget :type Actor%20Object%20Reference))
  (bind _astarget_point (Utilities|Casting|CastToTargetPoint NewTarget))
  (Variables|Default|SetCurrentTarget _astarget_point)
  (AI|Components|Blackboard|SetValueasObject (Variables|Default|GetCurrentBlackboard) (Variables|Default|GetAttackTargetKey) NewTarget))

(event EventBeginPlay
  (bind _blackboardcomponent (Class|AIController|UseBlackboard "/Game/Blueprints/LastStandBlueprints/Enemies/Controllers/BB_EnemyAttacker.BB_EnemyAttacker"))
  (Variables|Default|SetCurrentBlackboard _blackboardcomponent)
  (bind _outactors (Actor|GetAllActorsOfClass "/Script/Engine.TargetPoint"))
  (AI|Components|Blackboard|SetValueasObject (Variables|Default|GetCurrentBlackboard) (Variables|Default|GetAttackTargetKey) (Utilities|Array|Get(acopy) _outactors (Math|Random|RandomIntegerinRange 0 (- (Utilities|Array|Length _outactors) 1))))
  (AI|RunBehaviorTree "/Game/Blueprints/LastStandBlueprints/Enemies/Controllers/BT_EnemyAttacker.BT_EnemyAttacker"))

(fn ConstructionScript)