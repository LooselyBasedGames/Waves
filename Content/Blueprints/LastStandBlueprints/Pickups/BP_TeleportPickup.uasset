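; Teleport pickup that extends a parent pickup with a timed life after being dropped; the teleport itself is not handled here.
; Drop starts two timers: one attaches a looping-safe ice gate particle effect to the mesh after a short delay, the other destroys the actor when its lifetime ends.
; Picking it up again cancels both timers.
; Tick holds the spawned emitter at zero world rotation.
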(event Custom|DestroyPickup
  (Actor|DestroyActor))

(event Custom|SpawnEmitter
  (bind _returnvalue (Effects|SpawnEmitterAttached "/Game/InfinityBladeEffects/Effects/FX_Gates/ICE/P_Gate_Ice_Locked_01.P_Gate_Ice_Locked_01" (Variables|Default|GetStaticMesh) "None" "0, 0, 0" "0, 0, 0" "SnapToTarget" false))
  (Variables|Default|SetEmitter _returnvalue))

(event EventPickup
  (params (AttachTo :type Scene%20Component%20Object%20Reference))
  (bind _destroypickuphandler (Variables|Default|GetDestroyPickupHandler))
  (|CallParentFunction AttachTo)
  (if (Utilities|Time|IsValidTimerHandle _destroypickuphandler)
    (Utilities|Time|ClearandInvalidateTimerbyHandle _destroypickuphandler)
    (Utilities|Time|ClearandInvalidateTimerbyHandle (Variables|Default|GetSpawnEmitterHandler))))

(event EventDrop
  (|CallParentFunction)
  (bind _returnvalue (Utilities|Time|SetTimerbyEvent (delegate Custom|DestroyPickup) (Variables|Default|GetLifetime)))
  (Variables|Default|SetDestroyPickupHandler _returnvalue)
  (bind _returnvalue_2 (Utilities|Time|SetTimerbyEvent (delegate Custom|SpawnEmitter) 2.0))
  (Variables|Default|SetSpawnEmitterHandler _returnvalue_2))

(event EventTick
  (params (DeltaSeconds :type Float%20%28single-precision%29))
  (bind _emitter (Variables|Default|GetEmitter))
  (Utilities|IsValid _emitter
    (:Is%20Valid
      (Transformation|SetWorldRotation _emitter "0, 0, 0" false false))))

(fn ConstructionScript
  (|CallParentFunction))