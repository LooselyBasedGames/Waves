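; BP_Pickup is a physics object that VR motion controllers can pick up and drop.
; Pickup requires a BP_MotionController owner, re-parents the mesh to the root with a per-hand offset, disables physics, then snaps the root to the given component.
; Drop detaches the root and re-enables physics on the mesh.
; BeginPlay caches the mesh's relative location in MeshOffset, which these graphs never read.
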(event EventPickup
  (params (AttachTo :type Scene%20Component%20Object%20Reference))
  (bind _staticmesh (Variables|Default|GetStaticMesh))
  (bind _asbp_motion_controller (Utilities|Casting|CastToBP_MotionController (Components|GetOwner AttachTo)))
  (Transformation|AttachComponentToComponent _staticmesh (Variables|Default|GetDefaultSceneRoot) "None" "KeepRelative" "KeepRelative" "KeepRelative" true)
  (Transformation|SetRelativeLocationAndRotation (Variables|Default|GetStaticMesh) (CallFunction|GetLocationBasedonHand _asbp_motion_controller) "0, 0, 0" false true)
  (Physics|SetSimulatePhysics _staticmesh false)
  (Transformation|AttachComponentToComponent (Variables|Default|GetDefaultSceneRoot) AttachTo "None" "SnapToTarget" "SnapToTarget" "KeepRelative" false))

(event EventDrop
  (Transformation|DetachFromComponent (Variables|Default|GetDefaultSceneRoot) "KeepRelative" "KeepRelative" "KeepRelative" true)
  (Physics|SetSimulatePhysics (Variables|Default|GetStaticMesh) true))

(event EventBeginPlay
  (Variables|Default|SetMeshOffset (Variables|/Script/Engine.SceneComponent|GetRelativeLocation (Variables|Default|GetStaticMesh))))

(fn ConstructionScript)

(fn GetLocationBasedonHand
  (params (MotionController :type BP%20Motion%20Controller%20Object%20Reference))
  (switch Utilities|FlowControl|Switch|SwitchonEControllerHand (Variables|/Game/VirtualRealityBP/Blueprints/BP_MotionController.BP_MotionController_C|GetHand MotionController)
    (:Left
      (return (Variables|Default|GetLHOffset)))
    (:Right
      (return (Variables|Default|GetRHOffset)))
    (:Pad
      (return "0, 0, 0"))))