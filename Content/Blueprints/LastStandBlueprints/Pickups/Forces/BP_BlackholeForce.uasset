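; Black hole force actor that knocks down enemies within its radius in the Last Stand game.
; On spawn it attaches a sparks emitter and a gravity grenade explosion sound to its force component.
; Every tick it runs the inherited radius check, whose per-actor hook makes any enemy not already stunned fall down for slightly longer than the force's lifetime.
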(event EventBeginPlay
  (|CallParentFunction)
  (Effects|SpawnEmitterAttached "/Game/StarterContent/Particles/P_Sparks.P_Sparks" (Variables|Default|GetForceComponent) "None" "0, 0, 0" "0, 0, 0" "SnapToTargetIncludingScale")
  (Audio|SpawnSoundAttached "/Game/Sounds/Grenades/GravityGrenadeExplosion.GravityGrenadeExplosion" (Variables|Default|GetForceComponent) "None" "0, 0, 0" "0, 0, 0" "SnapToTargetIncludingScale" true))

(event EventTick
  (params (DeltaSeconds :type Float%20%28single-precision%29))
  (CallFunction|AffectActorsinRadius))

(event EventAffectActor
  (params (ActorToAffect :type Actor%20Object%20Reference))
  (bind _asbp_base_enemy_character (Utilities|Casting|CastToBP_BaseEnemyCharacter ActorToAffect))
  (if (not (Variables|/Game/Blueprints/LastStandBlueprints/Enemies/Characters/BP_BaseEnemyCharacter.BP_BaseEnemyCharacter_C|GetisStunned _asbp_base_enemy_character))
    (Default|FallDown _asbp_base_enemy_character (+ (Variables|Default|GetLifetime) 2.0))))

(fn ConstructionScript
  (|CallParentFunction))