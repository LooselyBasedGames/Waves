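; BP_BaseForce is a base actor for short-lived area forces that act on nearby actors and destroy themselves when their lifetime timer ends.
; AffectActorsInRadius runs a sphere overlap at the actor's location, using the ForceComponent radius and a configurable object type filter, and passes each hit to AffectActor.
; AffectActor is empty here as an override hook, and nothing in this graph triggers AffectActorsInRadius.
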(event Custom|Expire
  (Actor|DestroyActor))

(event Custom|AffectActor
  (params (ActorToAffect :type Actor%20Object%20Reference)))

(event Custom|AffectActorsInRadius
  (for _array_element (CallFunction|GetActorsinRadius)
    (CallFunction|AffectActor _array_element)))

(event EventBeginPlay
  (Utilities|Time|SetTimerbyEvent (delegate Custom|Expire) (Variables|Default|GetLifetime)))

(fn ConstructionScript)

(fn GetActorsinRadius
  (bind _outactors (Class|KismetSystemLibrary|SphereOverlapActorsNEW (Transformation|GetActorLocation) (Variables|/Script/Engine.RadialForceComponent|GetRadius (Variables|Default|GetForceComponent)) (LocalVariables|GetActorsToFind)))
  (return _outactors))