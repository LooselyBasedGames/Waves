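; BP_ExplosiveForce is a pickup force actor that sets off an explosion as soon as it begins play.
; On BeginPlay it runs the parent logic, affects actors in radius, spawns explosion particles and sound, then fires an impulse from its force component.
; Its AffectActor event kills any affected BP_BaseEnemyCharacter by calling Die and ignores all other actors.
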(event Custom|SpawnEffects
  (bind _returnvalue (Transformation|GetActorLocation))
  (Effects|SpawnEmitteratLocation "/Game/StarterContent/Particles/P_Explosion.P_Explosion" _returnvalue)
  (Audio|SpawnSoundatLocation "/Game/StarterContent/Audio/Explosion01.Explosion01" _returnvalue))

(event EventBeginPlay
  (|CallParentFunction)
  (CallFunction|AffectActorsinRadius)
  (CallFunction|SpawnEffects)
  (Class|RadialForceComponent|FireImpulse (Variables|Default|GetForceComponent)))

(event EventAffectActor
  (params (ActorToAffect :type Actor%20Object%20Reference))
  (bind _asbp_base_enemy_character (Utilities|Casting|CastToBP_BaseEnemyCharacter ActorToAffect))
  (Default|Die _asbp_base_enemy_character))

(fn ConstructionScript)