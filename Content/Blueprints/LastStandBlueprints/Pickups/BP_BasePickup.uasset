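; Base pickup actor that motion controllers grab and release, and that kills active enemy characters it hits.
; Pickup attaches it without physics and schedules its Parent spawner's Spawn; Drop restores physics and starts a self-destruct timer.
; Hits stop the enemy's AI and ragdoll it with force scaled by speed and mass.
; Kills score in Waves or Tower Defense game modes, with delayed self-destruction only in Waves.
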(event OnComponentHit(StaticMeshComponent)
  (params (HitComponent :type Primitive%20Component%20Object%20Reference) (OtherActor :type Actor%20Object%20Reference) (OtherComp :type Primitive%20Component%20Object%20Reference) (NormalImpulse :type Vector) (Hit :type Hit%20Result%20Structure%20%28by%20ref%29))
  (bind _returnvalue (Game|GetGameMode))
  (bind _asbp_enemy_character (Utilities|Casting|CastToBP_EnemyCharacter OtherActor))
  (if (Variables|/Game/Blueprints/BP_EnemyCharacter.BP_EnemyCharacter_C|GetIsActive _asbp_enemy_character)
    (bind _returnvalue_2 (AI|GetAIController _asbp_enemy_character))
    (AI|Navigation|StopMovement _returnvalue_2)
    (Variables|/Game/Blueprints/BP_EnemyCharacter.BP_EnemyCharacter_C|SetIsActive _asbp_enemy_character false)
    (Physics|SetSimulatePhysics (Variables|/Script/Engine.Character|GetMesh _asbp_enemy_character) true)
    (Physics|AddForce (Variables|/Script/Engine.Character|GetMesh _asbp_enemy_character) (* NormalImpulse (* (Math|Vector|VectorLength (Transformation|GetVelocity)) (* (Physics|GetMass (Variables|Debug|GetStaticMeshComponent)) (Variables|Default|GetForce)))) "None" false)
    (Default|Die _asbp_enemy_character)
    (bind _asbp_waves_game_mode (Utilities|Casting|CastToBP_WavesGameMode _returnvalue)
      (:then
        (Variables|/Game/Blueprints/BP_WavesGameMode.BP_WavesGameMode_C|SetEnemiesZoinked _asbp_waves_game_mode (+ (Variables|/Game/Blueprints/BP_WavesGameMode.BP_WavesGameMode_C|GetEnemiesZoinked _asbp_waves_game_mode) 1))
        (Default|RenderScore _asbp_waves_game_mode)
        (Utilities|Time|SetTimerbyFunctionName 0 "Destroy" 1.0))
      (:CastFailed
        (bind _asbp_tower_defense (Utilities|Casting|CastToBP_TowerDefense _returnvalue))
        (Variables|/Game/Blueprints/BP_TowerDefense.BP_TowerDefense_C|SetScore _asbp_tower_defense (+ (Variables|/Game/Blueprints/BP_TowerDefense.BP_TowerDefense_C|GetScore _asbp_tower_defense) 1))))))

(event Custom|Die
  (Actor|DestroyActor))

(event EventBeginPlay
  (Variables|Default|SetIsActive false))

(event Collision|EventActorBeginOverlap
  (params (OtherActor :type Actor%20Object%20Reference)))

(event EventTick
  (params (DeltaSeconds :type Float%20%28single-precision%29)))

(event EventPickup
  (params (AttachTo :type Scene%20Component%20Object%20Reference))
  (Variables|Default|SetIsActive false)
  (Physics|SetSimulatePhysics (Variables|Debug|GetStaticMeshComponent) false)
  (Transformation|AttachComponentToComponent (VehicleSound|GetRootComponent) AttachTo "None" "KeepWorld" "KeepWorld" "KeepWorld" false)
  (Utilities|IsValid (Variables|Default|GetParent)
    (:Is%20Valid
      (Utilities|Time|SetTimerbyFunctionName (Variables|Default|GetParent) "Spawn" 2.0)
      (Variables|Default|SetParent 0))))

(event EventDrop
  (Variables|Default|SetIsActive true)
  (Physics|SetSimulatePhysics (Variables|Debug|GetStaticMeshComponent) true)
  (Transformation|DetachFromActor "KeepWorld" "KeepWorld" "KeepWorld")
  (Utilities|Time|SetTimerbyEvent (delegate Custom|Die) 3e+01))

(fn ConstructionScript)

(fn Destroy
  (Actor|DestroyActor))