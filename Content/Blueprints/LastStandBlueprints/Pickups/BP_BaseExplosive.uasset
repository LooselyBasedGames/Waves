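; Base explosive pickup that detonates on a timer after being dropped.
; Extends the parent pickup's Pickup and Drop: dropping starts a CookTime countdown to Detonate, and picking it up clears that timer.
; Detonate spawns the ForceToSpawn actor at the static mesh's world transform, then destroys the explosive.
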(event Custom|Detonate
  (Game|SpawnActorfromClass (Variables|Default|GetForceToSpawn) (Transformation|GetWorldTransform (Variables|Default|GetStaticMesh)) "Undefined" 0 0)
  (Actor|DestroyActor))

(event EventPickup
  (params (AttachTo :type Scene%20Component%20Object%20Reference))
  (|CallParentFunction AttachTo)
  (Utilities|Time|ClearTimerbyFunctionName 0 "Detonate"))

(event EventDrop
  (|CallParentFunction)
  (Utilities|Time|SetTimerbyFunctionName 0 "Detonate" (Variables|Default|GetCookTime)))

(fn ConstructionScript
  (|CallParentFunction))