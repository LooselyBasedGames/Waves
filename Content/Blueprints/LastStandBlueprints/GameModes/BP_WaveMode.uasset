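; Wave game mode that tracks enemy deaths to advance rounds through BP_RoundManager.
; On BeginPlay it binds to every BP_WaveSpawner, then finds and initializes the round manager.
; Each spawned wave's enemies report deaths through event dispatchers to a kill counter.
; When kills reach the round's total wave template size times the spawner count, the counter resets and StartRound is called.
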(event Custom|Init
  (bind _outactors (Actor|GetAllActorsOfClass "/Game/Blueprints/LastStandBlueprints/Environment/BP_WaveSpawner.BP_WaveSpawner_C"))
  (CallFunction|BindtoSpawners _outactors)
  (bind _outactors_2 (Actor|GetAllActorsOfClass "/Game/Blueprints/LastStandBlueprints/Environment/BP_RoundManager.BP_RoundManager_C"))
  (bind _output_get (Variables|Default|SetRoundManager (Utilities|Array|Get(acopy) _outactors_2)))
  (Default|Init _output_get))

(event Custom|BindToEnemyDeath
  (params (Enemy :type BP%20Base%20Enemy%20Character%20Object%20Reference))
  (EventDispatchers|BindEventtoOnEnemyDie Enemy (delegate Custom|HandleEnemyDie)))

(event Custom|HandleEnemyDie
  (bind _result (Math|Integer|IncrementInt (Variables|Default|GetEnemiesKilled))
    (:%20%20
      (if (>= _result (CallFunction|GetMaxEnemies (Variables|/Game/Blueprints/LastStandBlueprints/Environment/BP_RoundManager.BP_RoundManager_C|GetCurrentRound (Variables|Default|GetRoundManager))))
        (Variables|Default|SetEnemiesKilled 0)
        (Default|StartRound (Variables|Default|GetRoundManager) 1.0)))))

(event Custom|BindToSpawners
  (params (Spawners :type Array%20of%20BP%20Wave%20Spawner%20Object%20References))
  (for _array_element Spawners
    (EventDispatchers|BindEventtoOnWaveSpawned _array_element (delegate Custom|HandleWaveSpawned))))

(event Custom|HandleWaveSpawned
  (params (Wave :type Array%20of%20BP%20Base%20Enemy%20Character%20Object%20References))
  (for _array_element Wave
    (CallFunction|BindtoEnemyDeath _array_element)))

(event EventBeginPlay
  (CallFunction|Init))

(fn ConstructionScript)

(fn GetMaxEnemies
  (params (Round :type Integer))
  (for _array_element (.waveconfigs (Utilities|Array|Get(acopy) (Variables|/Game/Blueprints/LastStandBlueprints/Environment/BP_RoundManager.BP_RoundManager_C|GetRoundConfigs (Variables|Default|GetRoundManager)) (- Round 1)))
    (LocalVariables|SetEnemyCount (+ (LocalVariables|GetEnemyCount) (Utilities|Array|Length (.WaveTemplate (Utilities|Struct|BreakWaveConfig _array_element))))))
  (Development|PrintString (Utilities|String|ToString(Integer) (* (LocalVariables|GetEnemyCount) (CallFunction|GetNumberOfSpawners))))
  (return (* (LocalVariables|GetEnemyCount) (CallFunction|GetNumberOfSpawners))))

(fn GetNumberOfSpawners
  (bind _outactors (Actor|GetAllActorsOfClass "/Game/Blueprints/LastStandBlueprints/Environment/BP_WaveSpawner.BP_WaveSpawner_C"))
  (return (Utilities|Array|Length _outactors)))