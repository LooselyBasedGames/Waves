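; Tower defense game mode that alternates timed prep and defense phases, with enemies arriving in waves.
; Defense broadcasts OnSpawnWave on a looping timer until the spawned count reaches the round maximum.
; It binds to every BP_EnemyWaveSpawner to count spawned enemies and track their destruction.
; Kills reaching that maximum trigger a delayed return to prep, though neither counter is reset here.
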(event Custom|Initialize
  (CallFunction|BeginPrepPhase)
  (bind _outactors (Actor|GetAllActorsOfClass "/Game/Blueprints/LastStandBlueprints/Environment/BP_EnemyWaveSpawner.BP_EnemyWaveSpawner_C"))
  (for _array_element _outactors
    (EventDispatchers|BindEventtoOnWaveSpawned _array_element (delegate Custom|HandleWaveSpawned))))

(event Custom|HandleWaveSpawned
  (params (WaveSize :type Integer) (EnemyWave :type Array%20of%20BP%20Base%20Enemy%20Character%20Object%20References))
  (Variables|Default|SetEnemiesSpawnedThisRound (+ WaveSize (Variables|Default|GetEnemiesSpawnedThisRound)))
  (for _array_element EnemyWave
    (Game|BindEventtoOnDestroyed _array_element (delegate Custom|HandleEnemyKilled))))

(event Custom|BeginDefensePhase
  (Default|CallOnSpawnWave)
  (bind _returnvalue (Utilities|Time|SetTimerbyEvent (delegate Custom|SpawnNextWave) (Variables|Default|GetTimeBetweenWaves) true))
  (Variables|Default|SetWaveSpawnHandler _returnvalue))

(event Custom|HandleEnemyKilled
  (params (DestroyedActor :type Actor%20Object%20Reference))
  (bind _result (Math|Integer|IncrementInt (Variables|Default|GetEnemiesKilled))
    (:%20%20
      (if (>= _result (Variables|Default|GetMaxEnemiesPerRound))
        (CallFunction|EndDefensePhase)))))

(event Custom|EndDefensePhase
  (Utilities|Time|SetTimerbyFunctionName 0 "BeginPrepPhase" 5.0))

(event Custom|SpawnNextWave
  (if (>= (Variables|Default|GetEnemiesSpawnedThisRound) (Variables|Default|GetMaxEnemiesPerRound))
    (Utilities|Time|ClearandInvalidateTimerbyHandle (Variables|Default|GetWaveSpawnHandler))
    (else
      (Default|CallOnSpawnWave))))

(event Custom|BeginPrepPhase
  (Utilities|Time|SetTimerbyFunctionName 0 "BeginDefensePhase" (Variables|Default|GetTimeBetweenRounds)))

(event EventBeginPlay
  (CallFunction|Initialize))

(fn ConstructionScript)