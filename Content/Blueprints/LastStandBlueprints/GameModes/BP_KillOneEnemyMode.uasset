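; Tutorial game mode whose objective is to kill one enemy before moving on to the next tutorial map, Factory2.
; On BeginPlay it restarts the player and binds to the death event of every BP_BaseEnemyCharacter already in the level.
; The first death fires the objective-completed dispatcher once, which fades out camera and audio and opens the next map on a timer just before the fade ends.
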(event Custom|ObjectiveCompleted
  (if (not (Variables|Default|GetisObjectiveCompleted))
    (Variables|Default|SetisObjectiveCompleted true)
    (Default|CallOnObjectiveCompleted)))

(event Custom|GoToNextTutorial
  (Game|OpenLevel(byName) (Variables|Default|GetNextTutorialMap)))

(event Custom|Init
  (Variables|Default|SetNextTutorialMap "Factory2")
  (Class|GameModeBase|RestartPlayer)
  (EventDispatchers|BindEventtoOnObjectiveCompleted (delegate Custom|HandleOnObjectiveCompleted))
  (bind _outactors (Actor|GetAllActorsOfClass "/Game/Blueprints/LastStandBlueprints/Enemies/Characters/BP_BaseEnemyCharacter.BP_BaseEnemyCharacter_C"))
  (for _array_element _outactors
    (EventDispatchers|BindEventtoOnEnemyDie _array_element (delegate Custom|ObjectiveCompleted))))

(event Custom|HandleOnObjectiveCompleted
  (CameraFades|StartCameraFade :self (Game|GetPlayerCameraManager 0) :ToAlpha 1.0 :Duration 3.0 :bShouldFadeAudio true)
  (Utilities|Time|SetTimerbyEvent (delegate Custom|GoToNextTutorial) 2.75))

(event EventBeginPlay
  (CallFunction|Init))

(fn ConstructionScript
  (|CallParentFunction))