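; Last Stand game mode that ends the game when every destructible attack target has been destroyed.
; On BeginPlay it counts all BP_BaseDestructibleObject actors and binds to each one's OnDestroyed, decrementing the count as they fall.
; GameOver extends the parent's logic, saves the score and any new high score to the waves game instance, then opens the game-over level after a short timer delay.
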(event Custom|InitGameMode
  (bind _outactors (Actor|GetAllActorsOfClass "/Game/Blueprints/LastStandBlueprints/Environment/BP_BaseDestructibleObject.BP_BaseDestructibleObject_C"))
  (for _array_element _outactors
    (bind _result (Math|Integer|IncrementInt (Variables|Default|GetAttackTargetsRemaining))
      (:%20%20
        (Variables|Default|SetAttackTargetsRemaining _result)
        (Game|BindEventtoOnDestroyed _array_element (delegate Custom|TowerDestroyed))))))

(event Custom|TowerDestroyed
  (params (DestroyedActor :type Actor%20Object%20Reference))
  (bind _result (Math|Integer|DecrementInt (Variables|Default|GetAttackTargetsRemaining))
    (:%20%20
      (bind _output_get (Variables|Default|SetAttackTargetsRemaining _result))
      (if (<= _output_get 0)
        (CallFunction|GameOver)))))

(event Custom|OpenGameOverMap
  (Game|OpenLevel(byName) (Variables|Default|GetGameOverLevel)))

(event EventBeginPlay
  (CallFunction|InitGameMode))

(event EventGameOver
  (bind _score (Variables|Default|GetScore))
  (|CallParentFunction)
  (Utilities|Time|SetTimerbyEvent (delegate Custom|OpenGameOverMap) 2.0)
  (bind _asbp_base_waves_game_instance (Utilities|Casting|CastToBP_BaseWavesGameInstance (Game|GetGameInstance)))
  (Default|SetScore _asbp_base_waves_game_instance _score)
  (if (< (Variables|/Game/Blueprints/LastStandBlueprints/GameInstances/BP_BaseWavesGameInstance.BP_BaseWavesGameInstance_C|GetHighScore _asbp_base_waves_game_instance) _score)
    (Variables|/Game/Blueprints/LastStandBlueprints/GameInstances/BP_BaseWavesGameInstance.BP_BaseWavesGameInstance_C|SetHighScore _asbp_base_waves_game_instance (Variables|Default|GetScore))))

(fn ConstructionScript)