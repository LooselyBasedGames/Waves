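; BP_TrapTutorialMode is the game mode for a trap tutorial level, completed when three enemies die.
; Tick scans for BP_BaseEnemyCharacter actors and binds each new one's OnEnemyDie once, tracked by object name in AlreadyRegistered.
; Reaching the kill target fires OnObjectiveCompleted, fades the camera out and opens Tutorial3 after a delay.
; Tick also rebinds OnObjectiveCompleted every frame to an empty handler.
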(event Custom|HandleEnemyDie
  (bind _result (Math|Integer|IncrementInt (Variables|Default|GetEnemiesKilled))
    (:%20%20
      (if (>= _result (Variables|Default|GetTargetEnemyKillCount))
        (Default|CallOnObjectiveCompleted)
        (CameraFades|StartCameraFade :self (Game|GetPlayerCameraManager 0) :ToAlpha 1.0 :Duration 2.0 :bHoldWhenFinished true)
        (Utilities|Time|SetTimerbyEvent (delegate Custom|OpenNextLevel) 3.0)))))

(event Custom|HandleObjectiveCompleted)

(event Custom|OpenNextLevel
  (Game|OpenLevel(byName) "Tutorial3"))

(event EventBeginPlay
  (Variables|Default|SetTargetEnemyKillCount 3)
  (Variables|Default|SetEnemiesKilled 0))

(event EventTick
  (params (DeltaSeconds :type Float%20%28single-precision%29))
  (EventDispatchers|BindEventtoOnObjectiveCompleted (delegate Custom|HandleObjectiveCompleted))
  (bind _outactors (Actor|GetAllActorsOfClass "/Game/Blueprints/LastStandBlueprints/Enemies/Characters/BP_BaseEnemyCharacter.BP_BaseEnemyCharacter_C"))
  (for _array_element _outactors
    (if (not (Utilities|Array|ContainsItem (Variables|Default|GetAlreadyRegistered) (Utilities|GetObjectName _array_element)))
      (Utilities|Array|Insert (Variables|Default|GetAlreadyRegistered) (Utilities|GetObjectName _array_element))
      (Development|PrintText "Binding event to OnEnemyDie...")
      (EventDispatchers|BindEventtoOnEnemyDie _array_element (delegate Custom|HandleEnemyDie)))))

(fn ConstructionScript
  (|CallParentFunction))