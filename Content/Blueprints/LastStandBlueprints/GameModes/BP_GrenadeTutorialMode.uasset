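; BP_GrenadeTutorialMode is the game mode for the grenade tutorial level, which completes once every enemy is killed.
; On BeginPlay it counts all BP_BaseEnemyCharacter actors and binds each death event to decrement that count.
; At zero it fires the objective-completed event, fades the camera out and opens the Tutorial3 level on a timer.
; Its own objective-completed handler is bound but empty.
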(event Custom|HandleEnemyDie
  (bind _result (Math|Integer|DecrementInt (Variables|Default|GetEnemyCount))
    (:%20%20
      (if (<= _result 0)
        (Default|CallOnObjectiveCompleted)
        (CameraFades|StartCameraFade :self (Game|GetPlayerCameraManager 0) :ToAlpha 1.0 :Duration 2.0 :bHoldWhenFinished true)
        (Utilities|Time|SetTimerbyEvent (delegate Custom|OpenNextLevel) 3.0)))))

(event Custom|HandleObjectiveCompleted)

(event Custom|OpenNextLevel
  (Game|OpenLevel(byName) "Tutorial3"))

(event EventBeginPlay
  (EventDispatchers|BindEventtoOnObjectiveCompleted (delegate Custom|HandleObjectiveCompleted))
  (bind _outactors (Actor|GetAllActorsOfClass "/Game/Blueprints/LastStandBlueprints/Enemies/Characters/BP_BaseEnemyCharacter.BP_BaseEnemyCharacter_C"))
  (Variables|Default|SetEnemyCount (Utilities|Array|Length _outactors))
  (for _array_element _outactors
    (EventDispatchers|BindEventtoOnEnemyDie _array_element (delegate Custom|HandleEnemyDie))))

(fn ConstructionScript
  (|CallParentFunction))