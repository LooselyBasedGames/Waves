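; BP_WaveSpawner spawns a wave of AI enemies around its own location.
; SpawnWave passes the wave's enemy classes to SpawnEnemies, which creates each one via SpawnEnemy at a random X/Y offset within SpawnRadius, ignoring collision failures.
; Each result is cast to BP_BaseEnemyCharacter, announced through OnEnemySpawned and added to Enemies.
; OnWaveSpawned then broadcasts that array.
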(event Custom|SpawnWave
  (params (Wave :type Array%20of%20BP%20Base%20Enemy%20Character%20Class%20References))
  (bind _enemywave (CallFunction|SpawnEnemies Wave))
  (Default|CallOnWaveSpawned _enemywave))

(fn ConstructionScript)

(fn SpawnEnemy
  (params (EnemyType :type BP%20Base%20Enemy%20Character%20Class%20Reference))
  (bind _returnvalue (AI|SpawnAIFromClass EnemyType 0 (+ (Transformation|GetActorLocation) (Math|Vector|MakeVector (Math|Conversions|ToFloat(Integer) (Math|Random|RandomIntegerinRange (* (Variables|Default|GetSpawnRadius) -1) (Variables|Default|GetSpawnRadius))) (Math|Conversions|ToFloat(Integer) (Math|Random|RandomIntegerinRange (* (Variables|Default|GetSpawnRadius) -1) (Variables|Default|GetSpawnRadius))) 0.0)) "0, 0, 0" true))
  (bind _asbp_base_enemy_character (Utilities|Casting|CastToBP_BaseEnemyCharacter _returnvalue)
    (:then
      (return _asbp_base_enemy_character))
    (:CastFailed
      (return 0))))

(fn SpawnEnemies
  (params (NewParam :type Array%20of%20BP%20Base%20Enemy%20Character%20Class%20References))
  (for _array_element NewParam
    (bind _enemy (CallFunction|SpawnEnemy _array_element))
    (Default|CallOnEnemySpawned _enemy)
    (Utilities|Array|Add (LocalVariables|GetEnemies) _enemy))
  (return (LocalVariables|GetEnemies)))