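; BP_PlayerPoint is a placed point actor that shows a fire circle particle effect at its location on demand.
; BeginPlay spawns the P_AOE_Fire_CircleAttack emitter there without auto-destroy and keeps it inactive.
; SpawnEffects activates that stored emitter and sets a timer by function name that calls DisableEffects to switch it off after a few seconds.
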(event Custom|SpawnEffects
  (Components|Activation|SetActive (Variables|Default|GetEmitter) true false)
  (Utilities|Time|SetTimerbyFunctionName 0 "DisableEffects" 3.5))

(event Custom|DisableEffects
  (Components|Activation|SetActive (Variables|Default|GetEmitter) false false))

(event EventBeginPlay
  (bind _returnvalue (Effects|SpawnEmitteratLocation "/Game/InfinityBladeEffects/Effects/FX_Mobile/Fire/combat/P_AOE_Fire_CircleAttack.P_AOE_Fire_CircleAttack" (Transformation|GetActorLocation) "0, 0, 0" false))
  (bind _output_get (Variables|Default|SetEmitter _returnvalue))
  (Components|Activation|SetActive _output_get false false))

(fn ConstructionScript)