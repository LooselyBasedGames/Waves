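; Tower defense enemy spawner actor that spawns waves of AI enemies at random navigable points around itself.
; On BeginPlay it binds to the tower defense game mode's begin-round event, which triggers an immediate wave and a looping timer at the supplied frequency.
; Each wave broadcasts its size through OnSpawnWave, then spawns that many pawns of the configured class.
; StopSpawning clears the timer.
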(event Custom|InitializeSpawner
  (params (WaveSpawnFrequency :type Float%20%28single-precision%29))
  (CallFunction|SpawnWave)
  (Utilities|Time|SetTimerbyFunctionName 0 "SpawnWave" WaveSpawnFrequency true))

(event Custom|SpawnWave
  (Default|CallOnSpawnWave (Variables|Default|GetWaveSize))
  (for _index (range 1 (Variables|Default|GetWaveSize))
    (AI|SpawnAIFromClass (Variables|Default|GetClassToSpawn) 0 (Class|NavigationSystem|GetRandomPointinNavigableRadius (Transformation|GetActorLocation) 4e+02) "0, 0, 0" false)))

(event Custom|StopSpawning
  (Utilities|Time|ClearTimerbyFunctionName 0 "SpawnWave"))

(event EventBeginPlay
  (bind _asbp_tower_defense_mode (Utilities|Casting|CastToBP_TowerDefenseMode (Game|GetGameMode)))
  (EventDispatchers|BindEventtoOnBeginRound _asbp_tower_defense_mode (delegate Custom|InitializeSpawner)))

(fn ConstructionScript)