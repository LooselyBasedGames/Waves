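; Wall trap that thrusts its surface out and kills enemies it strikes.
; Trigger arms the hit flag and slides TrapSurface by TravelDistance with a quick MoveComponentTo, then Reset disarms it and slides it back.
; While armed, component hits on a BP_BaseEnemyCharacter call Die.
; A timer meant to call DeactivatePhysics is left unconnected and never runs.
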(event OnComponentHit(TrapSurface)
  (params (HitComponent :type Primitive%20Component%20Object%20Reference) (OtherActor :type Actor%20Object%20Reference) (OtherComp :type Primitive%20Component%20Object%20Reference) (NormalImpulse :type Vector :default "0, 0, 0") (Hit :type Hit%20Result%20Structure%20%28by%20ref%29))
  (if (Variables|Default|GetShouldHit)
    (bind _asbp_base_enemy_character (Utilities|Casting|CastToBP_BaseEnemyCharacter OtherActor))
    (Default|Die _asbp_base_enemy_character)))

(event Custom|DeactivatePhysics
  (Physics|SetSimulatePhysics (Variables|Default|GetTrapSurface) false))

(event EventReset
  (Variables|Default|SetShouldHit false)
  (Components|MoveComponentTo (Variables|Default|GetTrapSurface) "0, 0, 0" "0, 0, 0" false false 0.1 false))

(event EventTrigger
  (Variables|Default|SetShouldHit true)
  (Components|MoveComponentTo (Variables|Default|GetTrapSurface) (Variables|Default|GetTravelDistance) "0, 0, 0" false false 0.1 false)
  (CallFunction|Reset))

(fn ConstructionScript)