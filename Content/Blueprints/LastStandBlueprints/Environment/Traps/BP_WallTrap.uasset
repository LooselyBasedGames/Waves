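; Wall trap, derived from a parent trap, that thrusts its Top component out on a physics-constraint spring to kill active enemies it hits.
; Trigger, also called on BeginPlay, drives the Top-to-Bottom constraint along Y with velocity and position targets if the trap is active.
; After the cooldown, Reset clears the drives and hit flag, then re-activates the trap two seconds later.
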(event OnComponentHit(Top)
  (params (HitComponent :type Primitive%20Component%20Object%20Reference) (OtherActor :type Actor%20Object%20Reference) (OtherComp :type Primitive%20Component%20Object%20Reference) (NormalImpulse :type Vector :default "0, 0, 0") (Hit :type Hit%20Result%20Structure%20%28by%20ref%29))
  (if (Variables|Default|GetShouldHit)
    (bind _asbp_enemy_character (Utilities|Casting|CastToBP_EnemyCharacter OtherActor))
    (if (Variables|/Game/Blueprints/BP_EnemyCharacter.BP_EnemyCharacter_C|GetIsActive _asbp_enemy_character)
      (Default|Die _asbp_enemy_character))))

(event Custom|Activate
  (Variables|Default|SetisActive true))

(event EventReset
  (bind _spring (Variables|Default|GetSpring))
  (Variables|Default|SetShouldHit false)
  (Class|PhysicsConstraintComponent|SetLinearVelocityTarget _spring (Math|Vector|MakeVector 0.0 0.0 0.0))
  (Class|PhysicsConstraintComponent|SetLinearVelocityDrive _spring false false false)
  (Class|PhysicsConstraintComponent|SetLinearPositionTarget _spring (Math|Vector|MakeVector 0.0 0.0 0.0))
  (Class|PhysicsConstraintComponent|SetLinearPositionDrive (Variables|Default|GetSpring) false false false)
  (Utilities|Time|SetTimerbyEvent (delegate Custom|Activate) 2.0))

(event EventTrigger
  (bind _spring (Variables|Default|GetSpring))
  (Variables|Default|SetShouldHit true)
  (if (CallFunction|IsTrapActive)
    (|CallParentFunction)
    (Class|PhysicsConstraintComponent|SetLinearVelocityDrive _spring false true false)
    (Class|PhysicsConstraintComponent|SetLinearVelocityTarget _spring (Math|Vector|MakeVector 0.0 (Variables|Default|GetSpringForce) 0.0))
    (Class|PhysicsConstraintComponent|SetLinearPositionDrive _spring false true false)
    (Class|PhysicsConstraintComponent|SetLinearPositionTarget (Variables|Default|GetSpring) (Math|Vector|MakeVector 0.0 (Variables|Default|GetMaxSpringHeight) 0.0))
    (Utilities|Time|SetTimerbyFunctionName 0 "Reset" (Variables|Default|GetCooldownTime))
    (else
      (Development|PrintString "Trap inactive"))))

(event EventBeginPlay
  (CallFunction|Trigger))

(fn ConstructionScript
  (|CallParentFunction)
  (Class|PhysicsConstraintComponent|SetConstrainedComponents (Variables|Default|GetSpring) (Variables|Default|GetTop) "None" (Variables|Default|GetBottom) "None"))