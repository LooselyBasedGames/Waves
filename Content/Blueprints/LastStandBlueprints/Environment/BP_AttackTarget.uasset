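; BP_AttackTarget is a damageable environment target that explodes when its health runs out.
; Its TakeDamage event subtracts the incoming amount from Health and calls Destroy once Health reaches zero or below.
; Destroy spawns an explosion particle and plays an explosion sound at the actor's location, then removes the actor.
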(event Custom|TakeDamage
  (params (Amount :type Integer))
  (Variables|Default|SetHealth (- (Variables|Default|GetHealth) Amount))
  (if (<= (Variables|Default|GetHealth) 0)
    (CallFunction|Destroy)))

(event Custom|Destroy
  (bind _returnvalue (Transformation|GetActorLocation))
  (Effects|SpawnEmitteratLocation "/Game/StarterContent/Particles/P_Explosion.P_Explosion" _returnvalue)
  (Audio|PlaySoundatLocation "/Game/StarterContent/Audio/Explosion01.Explosion01" _returnvalue)
  (Actor|DestroyActor))

(fn ConstructionScript)