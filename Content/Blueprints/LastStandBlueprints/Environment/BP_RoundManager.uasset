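; Round manager that drives the enemy round and wave loop, flashing the round number through the motion controller pawn.
; After a countdown, a looping timer hands successive RoundConfigs wave entries to all BP_WaveManagers until the round's waves run out.
; It binds to spawner events to count enemy deaths.
; The next round starts once kills reach the total wave template size multiplied by spawner count.
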(event Custom|CreateWave
  (for _array_element (Variables|Default|GetWaveManagers)
    (Default|SpawnWaves _array_element (CallFunction|GetNextWaveConfig (- (Variables|Default|GetCurrentRound) 1) (- (Variables|Default|GetCurrentWave) 1)))
    (Math|Integer|IncrementInt (Variables|Default|GetCurrentWave)))
  (if (Utilities|Time|IsValidTimerHandle (Variables|Default|GetInitialWaveSpawnHandle))
    (Utilities|Time|ClearandInvalidateTimerbyHandle (Variables|Default|GetInitialWaveSpawnHandle))))

(event Custom|ShowRoundCount
  (params (CurretnRound :type Integer))
  (bind _asmotion_controller_pawn (Utilities|Casting|CastToMotionControllerPawn (Game|Player|GetPlayerPawn 0)))
  (Default|CallOnShowRoundCount _asmotion_controller_pawn CurretnRound))

(event Custom|Init
  (bind _outactors (Actor|GetAllActorsOfClass "/Game/Blueprints/LastStandBlueprints/Environment/BP_WaveManager.BP_WaveManager_C"))
  (Variables|Default|SetWaveManagers _outactors)
  (CallFunction|BindtoEnemySpawned)
  (CallFunction|StartRound 1e+01))

(event Custom|StartRound
  (params (InitialSpawnCountdown :type Float%20%28single-precision%29))
  (Variables|Default|SetEnemiesKilled 0)
  (Variables|Default|SetCurrentWave 1)
  (bind _result (Math|Integer|IncrementInt (Variables|Default|GetCurrentRound))
    (:%20%20
      (CallFunction|ShowRoundCount _result)
      (bind _returnvalue (Utilities|Time|SetTimerbyFunctionName 0 "CreateInitialWave" InitialSpawnCountdown))
      (Variables|Default|SetInitialWaveSpawnHandle _returnvalue)
      (Utilities|Time|SetTimerbyEvent (delegate Custom|HideRoundCount) 2.0))))

(event Custom|BindToEnemySpawned
  (for _array_element (CallFunction|GetAllSpawners)
    (EventDispatchers|BindEventtoOnEnemySpawned _array_element (delegate Custom|HandleEnemySpawned))))

(event Custom|HandleEnemySpawned
  (params (Enemy :type Pawn%20Object%20Reference))
  (bind _asbp_base_enemy_character (Utilities|Casting|CastToBP_BaseEnemyCharacter Enemy))
  (EventDispatchers|BindEventtoOnEnemyDie _asbp_base_enemy_character (delegate Custom|HandleEnemyDie))
  (Development|PrintString "Enemy spawned"))

(event Custom|CreateInitialWave
  (CallFunction|CreateWave)
  (bind _returnvalue (Utilities|Time|SetTimerbyEvent (delegate Custom|SpawnNextWave) (.spawnfrequency (Utilities|Array|Get(acopy) (Variables|Default|GetRoundConfigs) (- (Variables|Default|GetCurrentRound) 1))) true))
  (Variables|Default|SetWaveeLoopSpawnHandle _returnvalue))

(event Custom|SpawnNextWave
  (if (CallFunction|AllWavesSpawned (Variables|Default|GetCurrentRound))
    (Utilities|Time|ClearandInvalidateTimerbyHandle (Variables|Default|GetWaveeLoopSpawnHandle))
    (else
      (CallFunction|CreateWave))))

(event Custom|HandleEnemyDie
  (Math|Integer|IncrementInt (Variables|Default|GetEnemiesKilled)
    (:%20%20
      (if (CallFunction|GetRoundCleared)
        (CallFunction|StartRound 1e+01)
        (Development|PrintString "Startnext round")
        (else
          (Development|PrintString "Enemy killed"))))))

(event Custom|HideRoundCount
  (bind _asmotion_controller_pawn (Utilities|Casting|CastToMotionControllerPawn (Game|Player|GetPlayerPawn 0)))
  (Default|CallOnHideRoundCount _asmotion_controller_pawn))

(event EventBeginPlay
  (CallFunction|Init))

(fn ConstructionScript)

(fn GetNextWaveConfig
  (params (RoundConfigIndex :type Integer) (WaveConfigIndex :type Integer))
  (return (Utilities|Array|Get(acopy) (.WaveConfigs (Utilities|Struct|BreakRoundConfig (Utilities|Array|Get(acopy) (Variables|Default|GetRoundConfigs) RoundConfigIndex))) WaveConfigIndex)))

(fn AllWavesSpawned
  (params (CurrentRound :type Integer))
  (return (< (Utilities|Array|Length (.waveconfigs (Utilities|Array|Get(acopy) (Variables|Default|GetRoundConfigs) (- CurrentRound 1)))) (Variables|Default|GetCurrentWave))))

(fn GetMaxEnemies
  (for _array_element (.waveconfigs (CallFunction|GetCurrentRoundConfig))
    (LocalVariables|SetEnemyCount (+ (LocalVariables|GetEnemyCount) (Utilities|Array|Length (Utilities|Struct|BreakWaveConfig _array_element)))))
  (bind _outactors (Actor|GetAllActorsOfClass "/Game/Blueprints/LastStandBlueprints/Environment/BP_WaveSpawner.BP_WaveSpawner_C"))
  (return (* (Utilities|Array|Length _outactors) (LocalVariables|GetEnemyCount))))

(fn GetCurrentRoundConfig
  (return (Utilities|Array|Get(acopy) (Variables|Default|GetRoundConfigs) (- (Variables|Default|GetCurrentRound) 1))))

(fn GetAllSpawners
  (bind _outactors (Actor|GetAllActorsOfClass "/Game/Blueprints/LastStandBlueprints/Environment/BP_WaveSpawner.BP_WaveSpawner_C"))
  (return _outactors))

(fn GetRoundCleared
  (return (>= (Variables|Default|GetEnemiesKilled) (CallFunction|GetMaxEnemies))))