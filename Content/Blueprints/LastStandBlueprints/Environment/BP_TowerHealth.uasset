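; BP_TowerHealth is an actor that displays the health of a referenced Tower as a percentage.
; It records the Tower's Health at BeginPlay as the maximum.
; UpdateHealth divides current Health by that maximum and writes the result to the HealthPercentValue text, once at BeginPlay and then by polling every Tick.
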(event EventBeginPlay
  (Variables|Default|SetTowerMaxHealth (Variables|/Game/Blueprints/LastStandBlueprints/Environment/BP_BaseDestructibleObject.BP_BaseDestructibleObject_C|GetHealth (Variables|Default|GetTower)))
  (CallFunction|UpdateHealth))

(event EventTick
  (params (DeltaSeconds :type Float%20%28single-precision%29))
  (CallFunction|UpdateHealth))

(fn ConstructionScript)

(fn UpdateHealth
  (Rendering|Components|TextRender|SetText (Variables|Default|GetHealthPercentValue) (Class|KismetTextLibrary|AsPercentFloat (/ (Variables|/Game/Blueprints/LastStandBlueprints/Environment/BP_BaseDestructibleObject.BP_BaseDestructibleObject_C|GetHealth (Variables|Default|GetTower)) (Variables|Default|GetTowerMaxHealth)) "HalfToEven")))