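; BP_AISpawner is a placed actor that periodically spawns AI pawns of a configurable class at its own location.
; A countdown timer started on BeginPlay triggers the first spawn, which then starts a looping timer that repeats Spawn at a set frequency.
; Each spawned pawn that casts to BP_BaseEnemyCharacter is broadcast through the AISpawned dispatcher.
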(event Custom|InitialSpawn
  (CallFunction|Spawn)
  (Utilities|Time|SetTimerbyFunctionName 0 "Spawn" (Variables|Default|GetSpawnFrequency) true))

(event EventSpawn
  (bind _aspawn (Utilities|Casting|CastToPawnClass (Variables|Default|GetClassToSpawn)))
  (bind _returnvalue (AI|SpawnAIFromClass _aspawn 0 (Transformation|GetActorLocation) "0, 0, 0" false))
  (bind _asbp_base_enemy_character (Utilities|Casting|CastToBP_BaseEnemyCharacter _returnvalue))
  (Default|CallAISpawned _asbp_base_enemy_character))

(event EventBeginPlay
  (Utilities|Time|SetTimerbyEvent (delegate Custom|InitialSpawn) (Variables|Default|GetInitialSpawnCountdown)))

(fn ConstructionScript)