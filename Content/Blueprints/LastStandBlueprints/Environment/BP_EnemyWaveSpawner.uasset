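; BP_EnemyWaveSpawner is a placed spawn point that creates waves of AI enemies around its location.
; On BeginPlay it binds to the SpawnManager's OnSpawnWave event, if the manager is valid, receiving enemy types and a wave size.
; Each spawn picks a random class and a random X/Y offset within Radius, giving a square area at the actor's height.
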(event Custom|SpawnEnemy
  (params (EnemyToSpawn :type BP%20Base%20Enemy%20Character%20Class%20Reference))
  ;[1 1 1] Spawns a specific enemy class at a random point in the radius
  (AI|SpawnAIFromClass EnemyToSpawn 0 (CallFunction|GetPointinRadius (Variables|Default|GetRadius)) "0, 0, 0" false))

(event Custom|HandleSpawnWave
  (params (EnemyWaveType :type Array%20of%20BP%20Base%20Enemy%20Character%20Class%20References) (Size :type Integer))
  (CallFunction|SpawnWave EnemyWaveType Size))

(event Custom|SpawnWave
  (params (EnemyTypes :type Array%20of%20BP%20Base%20Enemy%20Character%20Class%20References) (Size :type Integer))
  ;[1 1 1] Selects a random class from an array of enemy types to spawn 'n' times
  (for _index (range 1 Size)
    (CallFunction|SpawnEnemy (Utilities|Array|Get(acopy) EnemyTypes (Math|Random|RandomInteger (Utilities|Array|Length EnemyTypes))))))

(event EventBeginPlay
  (bind _spawnmanager (Variables|Default|GetSpawnManager))
  (Utilities|IsValid _spawnmanager
    (:Is%20Valid
      (EventDispatchers|BindEventtoOnSpawnWave _spawnmanager (delegate Custom|HandleSpawnWave)))))

(fn ConstructionScript)

(fn GetPointinRadius
  (params (Radius :type Integer))
  (return (+ (Transformation|GetActorLocation) (Math|Vector|MakeVector (Math|Conversions|ToFloat(Integer) (Math|Random|RandomIntegerinRange (* Radius -1) Radius)) (Math|Conversions|ToFloat(Integer) (Math|Random|RandomIntegerinRange (* Radius -1) Radius)) 0.0))))