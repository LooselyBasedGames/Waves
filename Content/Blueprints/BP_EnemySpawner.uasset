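; Enemy spawner that creates BP_EnemyCharacter actors at random BP_SpawnPoint locations in the level.
; BeginPlay starts a looping timer on SpawnEnemy, which clears it once the spawn count reaches MaxEnemies.
; Spawns adjust for collisions or fail if blocked, yet every attempt increments the count.
; A separate SpawnEnemies function loops SpawnEnemy for batch spawning but is not called within this Blueprint.
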(event EventBeginPlay
  (Utilities|Time|SetTimerbyFunctionName 0 "SpawnEnemy" (Math|Conversions|ToFloat(Integer) (Variables|Default|GetSpawnInterval)) true))

(event Collision|EventActorBeginOverlap
  (params (OtherActor :type Actor%20Object%20Reference)))

(event EventTick
  (params (DeltaSeconds :type Float%20%28single-precision%29)))

(fn ConstructionScript)

(fn SpawnEnemy
  (bind _transform (CallFunction|GetSpawnTransform))
  (Game|SpawnActorfromClass "/Game/Blueprints/BP_EnemyCharacter.BP_EnemyCharacter_C" _transform "AdjustIfPossibleButDontSpawnIfColliding" 0 0)
  (bind _output_get (Variables|Default|SetEnemySpawnCount (+ (Variables|Default|GetEnemySpawnCount) 1)))
  (if (>= _output_get (Variables|Default|GetMaxEnemies))
    (Utilities|Time|ClearTimerbyFunctionName 0 "SpawnEnemy")))

(fn GetSpawnTransform
  (bind _outactors (Actor|GetAllActorsOfClass "/Game/Blueprints/BP_SpawnPoint.BP_SpawnPoint_C"))
  (bind _output_get (LocalVariables|SetTransforms _outactors))
  (return (Transformation|GetActorTransform (Utilities|Array|Get(acopy) (LocalVariables|GetTransforms) (Math|Random|RandomIntegerinRange 0 (- (Utilities|Array|Length _output_get) 1))))))

(fn SpawnEnemies
  (for _index (range 0 (Variables|Default|GetMaxEnemies))
    (CallFunction|SpawnEnemy)))