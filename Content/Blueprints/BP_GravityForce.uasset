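; BP_GravityForce is a temporary force-field actor that shows a sparks effect and destroys itself and the effect when its Lifetime timer expires.
; Each Tick, it sphere-overlaps actors using its ForceComponent radius and passes them to AffectActor.
; AffectActor makes BP_EnemyCharacter actors fall down.
; Its BP_PickupCube physics step is chained behind the enemy cast, so cubes that fail that cast never reach it.
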(event EventBeginPlay
  (bind _returnvalue (Effects|SpawnEmitteratLocation "/Game/StarterContent/Particles/P_Sparks.P_Sparks" (Transformation|GetActorLocation)))
  (Variables|Default|SetEmitter _returnvalue)
  (Utilities|Time|SetTimerbyFunctionName 0 "Expire" (Variables|Default|GetLifetime)))

(event EventTick
  (params (DeltaSeconds :type Float%20%28single-precision%29))
  (bind _outactors (Class|KismetSystemLibrary|SphereOverlapActorsNEW (Transformation|GetActorLocation) (Variables|/Script/Engine.RadialForceComponent|GetRadius (Variables|Default|GetForceComponent)) (Variables|Default|GetObjectTypes)))
  (for _array_element _outactors
    (CallFunction|AffectActor _array_element)))

(fn ConstructionScript)

(fn Expire
  (Components|DestroyComponent (Variables|Default|GetEmitter))
  (Actor|DestroyActor))

(fn AffectActor
  (params (ActorToAffect :type Actor%20Object%20Reference))
  (bind _asbp_enemy_character (Utilities|Casting|CastToBP_EnemyCharacter ActorToAffect))
  (Default|FallDown _asbp_enemy_character)
  (bind _asbp_pickup_cube (Utilities|Casting|CastToBP_PickupCube ActorToAffect))
  (Physics|SetSimulatePhysics (Variables|/Script/Engine.StaticMeshActor|GetStaticMeshComponent _asbp_pickup_cube) true))