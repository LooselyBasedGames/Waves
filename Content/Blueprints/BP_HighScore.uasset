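; BP_HighScore is an actor that displays the game's high score on its HighScore text component.
; On BeginPlay it casts the game instance to BP_WavesGameInstance, converts the stored HighScore to text and sets it on the component.
; The cast and set are performed twice in succession with the same result, and the text is not refreshed afterward.
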(event EventBeginPlay
  (bind _asbp_waves_game_instance (Utilities|Casting|CastToBP_WavesGameInstance (Game|GetGameInstance))
    (:then
      (Rendering|Components|TextRender|SetText (Variables|Default|GetHighScore) (Utilities|Text|ToText(Integer) (Variables|/Game/Blueprints/BP_WavesGameInstance.BP_WavesGameInstance_C|GetHighScore _asbp_waves_game_instance))))
    (:CastFailed
      _))
  (bind _asbp_waves_game_instance_2 (Utilities|Casting|CastToBP_WavesGameInstance (Game|GetGameInstance)))
  (Rendering|Components|TextRender|SetText (Variables|Default|GetHighScore) (Utilities|Text|ToText(Integer) (Variables|/Game/Blueprints/BP_WavesGameInstance.BP_WavesGameInstance_C|GetHighScore _asbp_waves_game_instance_2))))

(event Collision|EventActorBeginOverlap
  (params (OtherActor :type Actor%20Object%20Reference)))

(event EventTick
  (params (DeltaSeconds :type Float%20%28single-precision%29)))

(fn ConstructionScript)