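; BP_ExplosiveForce is an explosion actor that knocks physics objects around and kills enemies within its radius.
; On BeginPlay it spawns explosion particles and sound, then finds nearby actors with a sphere overlap sized by its ForceComponent.
; Each actor with a mesh component starts simulating physics, and any BP_EnemyCharacter among them dies.
; The ForceComponent then fires its impulse, so newly simulated bodies get pushed by the blast.
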(event EventBeginPlay
  (bind _returnvalue (Transformation|GetActorLocation))
  (Effects|SpawnEmitteratLocation "/Game/StarterContent/Particles/P_Explosion.P_Explosion" _returnvalue)
  (Audio|PlaySoundatLocation "/Game/StarterContent/Audio/Explosion01.Explosion01" _returnvalue)
  (bind _outactors (Class|KismetSystemLibrary|SphereOverlapActorsNEW _returnvalue (Variables|/Script/Engine.RadialForceComponent|GetRadius (Variables|Default|GetForceComponent)) (Variables|Default|GetObjectsToFind)))
  (for _array_element _outactors
    (CallFunction|AffectActor _array_element))
  (Class|RadialForceComponent|FireImpulse (Variables|Default|GetForceComponent)))

(fn ConstructionScript)

(fn AffectActor
  (params (ActorToAffect :type Actor%20Object%20Reference))
  (bind _returnvalue (Actor|GetComponentbyClass ActorToAffect "/Script/Engine.MeshComponent"))
  (Utilities|IsValid _returnvalue
    (:Is%20Valid
      (Physics|SetSimulatePhysics _returnvalue true)
      (bind _asbp_enemy_character (Utilities|Casting|CastToBP_EnemyCharacter ActorToAffect))
      (Default|Die _asbp_enemy_character))))