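; AI controller for BP_EnemyCharacter that sends the pawn toward a randomly chosen BP_Target actor.
; FindTarget runs on possess and BeginPlay, and again when the bound target is destroyed or Tick finds it invalid.
; FallDown halts movement and ragdolls the pawn, then a timer calls GetUp to restore capsule and mesh and resume seeking.
; A separate TargetAcquired event writes a target to the EnemyBB blackboard and runs EnemyBT.
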(event Custom|TargetAcquired
  (params (Target :type BP%20Target%20Object%20Reference))
  ;[1 1 1] Sets the target on the black board
  (bind _blackboardcomponent (Class|AIController|UseBlackboard "/Game/Blueprints/EnemyBB.EnemyBB"))
  (AI|Components|Blackboard|SetValueasObject _blackboardcomponent (Variables|Default|GetTarget) Target)
  (AI|RunBehaviorTree "/Game/Blueprints/EnemyBT.EnemyBT"))

(event Custom|TargetDestroyed
  (params (DestroyedActor :type Actor%20Object%20Reference))
  (bind _asbp_enemy_character (Utilities|Casting|CastToBP_EnemyCharacter (Pawn|GetControlledPawn)))
  (Variables|/Game/Blueprints/BP_EnemyCharacter.BP_EnemyCharacter_C|SetisAttacking _asbp_enemy_character false)
  (Variables|Default|SetCurrentTarget 0)
  (CallFunction|FindTarget))

(event Custom|FindTarget
  (bind _output_get (Variables|Default|SetCurrentTarget (CallFunction|GetRandomTarget)))
  (AI|AIMoveTo 0 "0, 0, 0" _output_get 5.0 false))

(event Custom|FallDown
  (AI|Navigation|StopMovement)
  (bind _asbp_enemy_character (Utilities|Casting|CastToBP_EnemyCharacter (Pawn|GetControlledPawn)))
  (Variables|Default|SetLocationOnFallDown (Variables|/Script/Engine.SceneComponent|GetRelativeLocation (Variables|/Script/Engine.Character|GetCapsuleComponent _asbp_enemy_character)))
  (Variables|Default|SetRotationAtFallDown (Variables|/Script/Engine.SceneComponent|GetRelativeRotation (Variables|/Script/Engine.Character|GetMesh _asbp_enemy_character)))
  (Physics|SetSimulatePhysics (Variables|/Script/Engine.Character|GetCapsuleComponent _asbp_enemy_character) true)
  (Class|SkeletalMeshComponent|SetAllBodiesBelowSimulatePhysics (Variables|/Script/Engine.Character|GetMesh _asbp_enemy_character) (Utilities|String|StringToName (Utilities|String|MakeLiteralString "root")) true false)
  (Utilities|Time|SetTimerbyEvent (delegate Custom|GetUp) 6.0))

(event Custom|GetUp
  (Variables|Default|SetShouldGetUp true)
  (bind _asbp_enemy_character (Utilities|Casting|CastToBP_EnemyCharacter (Pawn|GetControlledPawn)))
  (Physics|SetSimulatePhysics (Variables|/Script/Engine.Character|GetMesh _asbp_enemy_character) false)
  (Physics|SetSimulatePhysics (Variables|/Script/Engine.Character|GetCapsuleComponent _asbp_enemy_character) false)
  (Transformation|AttachComponentToComponent (Variables|/Script/Engine.Character|GetCapsuleComponent _asbp_enemy_character) (VehicleSound|GetRootComponent _asbp_enemy_character) "None" "SnapToTarget" "SnapToTarget" "SnapToTarget" false)
  (Transformation|AttachComponentToComponent (Variables|/Script/Engine.Character|GetMesh _asbp_enemy_character) (Variables|/Script/Engine.Character|GetCapsuleComponent _asbp_enemy_character) "None" "SnapToTarget" "SnapToTarget" "SnapToTarget" false)
  (Transformation|SetRelativeLocationAndRotation (Variables|/Script/Engine.Character|GetCapsuleComponent _asbp_enemy_character) (Math|Vector|MakeVector (.x (Transformation|GetWorldLocation (Variables|/Script/Engine.Character|GetCapsuleComponent _asbp_enemy_character))) (.y (Transformation|GetWorldLocation (Variables|/Script/Engine.Character|GetCapsuleComponent _asbp_enemy_character))) (.z (Transformation|GetWorldLocation (Variables|/Script/Engine.Character|GetCapsuleComponent _asbp_enemy_character)))) "0, 0, 0" false true)
  (Transformation|SetRelativeLocationAndRotation (Variables|/Script/Engine.Character|GetMesh _asbp_enemy_character) "0, 0,-90.000000" (Variables|Default|GetRotationAtFallDown) false true)
  (CallFunction|FindTarget))

(event EventOnPossess
  (params (PossessedPawn :type Pawn%20Object%20Reference))
  (CallFunction|FindTarget)
  (Game|BindEventtoOnDestroyed (Variables|Default|GetCurrentTarget) (delegate Custom|TargetDestroyed)))

(event EventTick
  (params (DeltaSeconds :type Float%20%28single-precision%29))
  (if (not (Utilities|IsValid (Variables|Default|GetCurrentTarget)))
    (CallFunction|FindTarget)))

(event EventBeginPlay
  (CallFunction|FindTarget)
  (Game|BindEventtoOnDestroyed (Variables|Default|GetCurrentTarget) (delegate Custom|TargetDestroyed)))

(fn ConstructionScript)

(fn GetRandomTarget
  (bind _outactors (Actor|GetAllActorsOfClass "/Game/Blueprints/BP_Target.BP_Target_C"))
  (bind _output_get (LocalVariables|SetTargets _outactors))
  (return (Utilities|Array|Get(acopy) (LocalVariables|GetTargets) (Math|Random|RandomIntegerinRange 0 (- (Utilities|Array|Length _output_get) 1)))))