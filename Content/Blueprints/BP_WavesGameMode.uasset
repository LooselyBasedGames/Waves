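; Wave game mode that shows kill ("zoinked") and leak counts and ends the game when too many enemies pass.
; BeginPlay takes the first two BP_Text actors by array order as the green score and red passed displays, refreshed through RenderScore and RenderLoss.
; Tick polls the passed limit, then saves current and high score to BP_WavesGameInstance and opens the GameOver level.
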(event Custom|RenderScore
  (bind _score (Variables|Default|GetScore))
  (bind _textrender (Variables|/Game/Blueprints/BP_Text.BP_Text_C|GetTextRender _score))
  (if (Utilities|IsValid (Variables|Default|GetScore))
    (Rendering|Components|TextRender|SetTextRenderColor _textrender (Math|Conversions|ToColor(LinearColor) (Math|Color|MakeColor 0.0 1.0 0.0)))
    (Rendering|Components|TextRender|SetText _textrender (Utilities|Text|ToText(Integer) (Variables|Default|GetEnemiesZoinked)))))

(event Custom|RenderLoss
  (bind _passed (Variables|Default|GetPassed))
  (bind _textrender (Variables|/Game/Blueprints/BP_Text.BP_Text_C|GetTextRender _passed))
  (if (Utilities|IsValid (Variables|Default|GetPassed))
    (Rendering|Components|TextRender|SetTextRenderColor _textrender (Math|Conversions|ToColor(LinearColor) (Math|Color|MakeColor 1.0 0.0 0.0)))
    (Rendering|Components|TextRender|SetText _textrender (Utilities|Text|ToText(Integer) (Variables|Default|GetEnemiesPassed)))))

(event EventBeginPlay
  (bind _outactors (Actor|GetAllActorsOfClass "/Game/Blueprints/BP_Text.BP_Text_C"))
  (bind _output_get (Variables|Default|SetTexts _outactors))
  (Variables|Default|SetScore (Utilities|Array|Get(acopy) _output_get))
  (CallFunction|RenderScore)
  (Variables|Default|SetPassed (Utilities|Array|Get(acopy) (Variables|Default|GetTexts) 1))
  (CallFunction|RenderLoss))

(event EventTick
  (params (DeltaSeconds :type Float%20%28single-precision%29))
  (if (>= (Variables|Default|GetEnemiesPassed) (Variables|Default|GetMaxEnemiesAllowed))
    (bind _asbp_waves_game_instance (Utilities|Casting|CastToBP_WavesGameInstance (Game|GetGameInstance)))
    (bind _output_get (Variables|/Game/Blueprints/BP_WavesGameInstance.BP_WavesGameInstance_C|SetCurrentScore _asbp_waves_game_instance (Variables|Default|GetEnemiesZoinked)))
    (if (> _output_get (Variables|/Game/Blueprints/BP_WavesGameInstance.BP_WavesGameInstance_C|GetHighScore _asbp_waves_game_instance))
      (Variables|/Game/Blueprints/BP_WavesGameInstance.BP_WavesGameInstance_C|SetHighScore _asbp_waves_game_instance (Variables|Default|GetEnemiesZoinked)))
    (CallFunction|LoseGame)))

(fn ConstructionScript)

(fn LoseGame
  (Game|OpenLevel(byName) "GameOver"))