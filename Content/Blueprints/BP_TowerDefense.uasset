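; BP_TowerDefense runs the tower defense match, tracking survival time and ending the game when every tower is destroyed.
; On BeginPlay it gathers the timer and tower actors and binds each tower's OnDestroyed event to LoseGame, while Tick copies the first timer's seconds.
; When the last tower falls, it saves time and score to BP_WavesGameInstance, updates the best records, and opens the game over level.
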(event Custom|UpdateCurrentTime
  (bind _timers (Variables|Default|GetTimers))
  (bind _item (Utilities|Array|Get(acopy) _timers))
  (Utilities|IsValid _item
    (:Is%20Valid
      (Variables|Default|SetCurrentTime (Variables|/Game/Blueprints/Environment/BP_Timer.BP_Timer_C|GetSeconds _item)))))

(event Custom|LoseGame
  (params (DestroyedActor :type Actor%20Object%20Reference))
  (bind _asbp_tower (Utilities|Casting|CastToBP_Tower DestroyedActor))
  ;[1 1 1] Remove the tower that got destroyed from our array then check the length. If its 0 then the game is over and the score is set
  (Utilities|Array|RemoveItem (Variables|Default|GetTowers) _asbp_tower)
  (if (< (Utilities|Array|Length (Variables|Default|GetTowers)) 1)
    (bind _asbp_waves_game_instance (Utilities|Casting|CastToBP_WavesGameInstance (Game|GetGameInstance)))
    (Variables|/Game/Blueprints/BP_WavesGameInstance.BP_WavesGameInstance_C|SetCurrentTime _asbp_waves_game_instance (Variables|Default|GetCurrentTime))
    (if (< (Variables|/Game/Blueprints/BP_WavesGameInstance.BP_WavesGameInstance_C|GetBestTime _asbp_waves_game_instance) (Variables|Default|GetCurrentTime))
      (Variables|/Game/Blueprints/BP_WavesGameInstance.BP_WavesGameInstance_C|SetBestTime _asbp_waves_game_instance (Variables|Default|GetCurrentTime)))
    (bind _output_get (Variables|/Game/Blueprints/BP_WavesGameInstance.BP_WavesGameInstance_C|SetCurrentScore _asbp_waves_game_instance (Variables|Default|GetScore)))
    (if (> _output_get (Variables|/Game/Blueprints/BP_WavesGameInstance.BP_WavesGameInstance_C|GetHighScore _asbp_waves_game_instance))
      (Variables|/Game/Blueprints/BP_WavesGameInstance.BP_WavesGameInstance_C|SetHighScore _asbp_waves_game_instance (Variables|Default|GetScore))
      (Game|OpenLevel(byName) "GameOverTowerDefense")
      (else
        (Game|OpenLevel(byName) "GameOverTowerDefense")))))

(event EventBeginPlay
  (bind _outactors (Actor|GetAllActorsOfClass "/Game/Blueprints/Environment/BP_Timer.BP_Timer_C"))
  (Variables|Default|SetTimers _outactors)
  (bind _outactors_2 (Actor|GetAllActorsOfClass "/Game/Blueprints/Environment/BP_Tower.BP_Tower_C"))
  (bind _output_get (Variables|Default|SetTowers _outactors_2))
  (for _array_element _output_get
    (Game|BindEventtoOnDestroyed _array_element (delegate Custom|LoseGame))))

(event EventTick
  (params (DeltaSeconds :type Float%20%28single-precision%29))
  (CallFunction|UpdateCurrentTime))

(fn ConstructionScript)