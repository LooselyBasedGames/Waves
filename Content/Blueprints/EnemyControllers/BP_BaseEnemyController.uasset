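; Base AI controller for enemy characters, running a simple state machine over moving, attacking, falling and standing up.
; On BeginPlay it picks a random BP_MoveTarget, caches the controlled enemy character and enters the initial state.
; SetState runs exit and enter handlers that delegate movement, attack, fall and get-up actions to the character.
; Falling advances to standing up on a timer using the character's fall-down time.
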(event EventBeginPlay
  (Variables|Default|SetCurrentTarget (CallFunction|FindRandomTarget))
  (bind _asbp_base_enemy_character (Utilities|Casting|CastToBP_BaseEnemyCharacter (Pawn|GetControlledPawn)))
  (Variables|Default|SetControlledEnemyCharacter _asbp_base_enemy_character)
  (CallFunction|SetState (Variables|Default|GetInitialState)))

(fn ConstructionScript)

(fn FindRandomTarget
  (bind _outactors (Actor|GetAllActorsOfClass "/Game/Blueprints/Environment/BP_MoveTarget.BP_MoveTarget_C"))
  (bind _output_get (LocalVariables|SetAllTargets _outactors))
  (return (Utilities|Array|Get(acopy) _output_get (Math|Random|RandomIntegerinRange 0 (- (Utilities|Array|Length (LocalVariables|GetAllTargets)) 1)))))

(fn SetState
  (params (NewState :type BaseEnemyStates%20Enum))
  (CallFunction|ExitState (Variables|Default|GetCurrentState))
  (bind _output_get (Variables|Default|SetCurrentState NewState))
  (switch Utilities|FlowControl|Switch|SwitchonBaseEnemyStates _output_get
    (:NewEnumerator0
      (CallFunction|EnterMovingState))
    (:NewEnumerator1
      (CallFunction|EnterAttackingState))
    (:NewEnumerator2
      (CallFunction|EnterFallingState))
    (:NewEnumerator3
      (CallFunction|EnterStandingUpState))))

(fn EnterMovingState
  (bind _controlledenemycharacter (Variables|Default|GetControlledEnemyCharacter))
  (Utilities|IsValid _controlledenemycharacter
    (:Is%20Valid
      (Utilities|IsValid (Variables|Default|GetCurrentTarget)
        (:Is%20Valid
          (Default|MovetoTarget _controlledenemycharacter (Variables|Default|GetCurrentTarget) 0.0))
        (:Is%20Not%20Valid
          (bind _output_get (Variables|Default|SetCurrentTarget (CallFunction|FindRandomTarget)))
          (Default|MovetoTarget (Variables|Default|GetControlledEnemyCharacter) _output_get 0.0))))))

(fn EnterAttackingState
  (Variables|Default|SetIsAttacking true)
  (bind _asbp_move_target (Utilities|Casting|CastToBP_MoveTarget (Variables|Default|GetCurrentTarget)))
  (Default|BeginAttack (Variables|Default|GetControlledEnemyCharacter) _asbp_move_target))

(fn ExitState
  (params (PreviousState :type BaseEnemyStates%20Enum))
  (switch Utilities|FlowControl|Switch|SwitchonBaseEnemyStates PreviousState
    (:NewEnumerator0
      (CallFunction|ExitMovingState))
    (:NewEnumerator1
      (CallFunction|ExitAttackState))))

(fn ExitMovingState
  (Default|StopMoving (Variables|Default|GetControlledEnemyCharacter)))

(fn ExitAttackState
  (Variables|Default|SetIsAttacking false))

(fn EnterFallingState
  (Default|StartFalling (Variables|Default|GetControlledEnemyCharacter))
  (Utilities|Time|SetTimerbyFunctionName 0 "StartStandingUp" (Variables|/Game/Blueprints/EnemyCharacters/BP_BaseEnemyCharacter.BP_BaseEnemyCharacter_C|GetFallDownTime (Variables|Default|GetControlledEnemyCharacter))))

(fn StartStandingUp
  (CallFunction|SetState "NewEnumerator3"))

(fn EnterStandingUpState
  (Default|GetUp (Variables|Default|GetControlledEnemyCharacter)))