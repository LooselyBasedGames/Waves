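; BP_AttackTarget is an environment target actor that can be damaged and destroyed.
; Its TakeDamage event subtracts the incoming amount from Health, prints the new value, and calls Destroy once Health reaches zero or below.
; Destroy spawns the P_Explosion emitter and calls PlaySoundAtLocation, with no sound asset shown, at the actor's location, then removes the actor.
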(event Custom|TakeDamage
  (params (Amount :type Integer))
  (Variables|Default|SetHealth (- (Variables|Default|GetHealth) Amount))
  (Development|PrintString (Utilities|String|ToString(Integer) (Variables|Default|GetHealth)))
  (if (<= (Variables|Default|GetHealth) 0)
    (CallFunction|Destroy)))

(event Custom|Destroy
  (bind _returnvalue (Transformation|GetActorLocation))
  (Effects|SpawnEmitteratLocation "/Game/StarterContent/Particles/P_Explosion.P_Explosion" _returnvalue)
  (Audio|PlaySoundatLocation 0 _returnvalue)
  (Actor|DestroyActor))

(fn ConstructionScript)