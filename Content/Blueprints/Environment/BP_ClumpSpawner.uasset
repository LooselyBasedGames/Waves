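; BP_ClumpSpawner is an environment actor that spawns a clump of actors at nearby spawn points.
; Its Spawn function runs a sphere overlap at its location, filtered to BP_SpawnPoint, and spawns ActorToSpawn at each hit's transform, adjusting for collisions but always spawning.
; Spawned actors accumulate in ActorsSpawned, which the function returns; nothing in the file calls it, so an outside caller triggers spawning.
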(event EventTick
  (params (DeltaSeconds :type Float%20%28single-precision%29)))

(fn ConstructionScript)

(fn Spawn
  (bind _outactors (Class|KismetSystemLibrary|SphereOverlapActorsNEW (Transformation|GetActorLocation) (Variables|Default|GetRadius) (Variables|Default|GetObjectTypes) "/Game/Blueprints/BP_SpawnPoint.BP_SpawnPoint_C"))
  (for _array_element _outactors
    (bind _returnvalue (Game|SpawnActorfromClass (Variables|Default|GetActorToSpawn) (Transformation|GetActorTransform _array_element) "AdjustIfPossibleButAlwaysSpawn" 0 0))
    (Utilities|Array|Add (LocalVariables|GetActorsSpawned) _returnvalue))
  (return (LocalVariables|GetActorsSpawned)))