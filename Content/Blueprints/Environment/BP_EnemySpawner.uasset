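; Enemy spawner actor that fills the level with enemies on two looping timers started at BeginPlay.
; One timer spawns a BP_EnemyCharacter at a random BP_SpawnPoint; the other calls Spawn on a random BP_ClumpSpawner from a list cached at BeginPlay.
; Both add to a shared enemy count, and each timer clears itself when its own spawn finds that count at or above MaxEnemies.
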(event Custom|GetClumps
  (bind _outactors (Actor|GetAllActorsOfClass "/Game/Blueprints/Environment/BP_ClumpSpawner.BP_ClumpSpawner_C"))
  (Variables|Default|SetSpawnClumps _outactors))

(event Custom|SpawnClump
  (bind _clump (CallFunction|GetRandomClump))
  (Utilities|IsValid _clump
    (:Is%20Valid
      (bind _actors (Default|Spawn _clump))
      (bind _output_get (Variables|Default|SetEnemySpawnCount (+ (Utilities|Array|Length _actors) (Variables|Default|GetEnemySpawnCount))))
      (Development|PrintString (Utilities|String|ToString(Integer) _output_get))
      (if (>= _output_get (Variables|Default|GetMaxEnemies))
        (Utilities|Time|ClearTimerbyFunctionName 0 "SpawnClump")))))

(event EventBeginPlay
  (CallFunction|GetClumps)
  (Utilities|Time|SetTimerbyFunctionName 0 "SpawnEnemy" (Math|Conversions|ToFloat(Integer) (Variables|Default|GetSpawnInterval)) true)
  (Utilities|Time|SetTimerbyFunctionName 0 "SpawnClump" (Variables|Default|GetClumpSpawnFrequency) true))

(event Collision|EventActorBeginOverlap
  (params (OtherActor :type Actor%20Object%20Reference)))

(event EventTick
  (params (DeltaSeconds :type Float%20%28single-precision%29)))

(fn ConstructionScript)

(fn SpawnEnemy
  (bind _transform (CallFunction|GetSpawnTransform))
  (Game|SpawnActorfromClass "/Game/Blueprints/BP_EnemyCharacter.BP_EnemyCharacter_C" _transform "AdjustIfPossibleButDontSpawnIfColliding" 0 0)
  (bind _output_get (Variables|Default|SetEnemySpawnCount (+ (Variables|Default|GetEnemySpawnCount) 1)))
  (if (>= _output_get (Variables|Default|GetMaxEnemies))
    (Utilities|Time|ClearTimerbyFunctionName 0 "SpawnEnemy")))

(fn GetSpawnTransform
  (bind _outactors (Actor|GetAllActorsOfClass "/Game/Blueprints/BP_SpawnPoint.BP_SpawnPoint_C"))
  (bind _output_get (LocalVariables|SetTransforms _outactors))
  (return (Transformation|GetActorTransform (Utilities|Array|Get(acopy) (LocalVariables|GetTransforms) (Math|Random|RandomIntegerinRange 0 (- (Utilities|Array|Length _output_get) 1))))))

(fn GetRandomClump
  (return (Utilities|Array|Get(acopy) (Variables|Default|GetSpawnClumps) (Math|Random|RandomIntegerinRange 0 (- (Utilities|Array|Length (Variables|Default|GetSpawnClumps)) 1)))))