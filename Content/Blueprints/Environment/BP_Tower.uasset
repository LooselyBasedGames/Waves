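; BP_Tower is a destructible tower that takes damage from enemies and shows its health on a three-box child-actor health bar.
; Each hit lowers TowerHealth and swaps box materials to damaged or depleted as it drops below stepped thresholds.
; Surviving hits record unique BP_EnemyCharacter attackers in CurrentAttackers.
; A lethal hit from an enemy clears only that attacker's target and destroys the tower after a one-second timer.
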(event EventBeginPlay
  (Variables|Default|SetMaxHealth (Variables|Default|GetTowerHealth)))

(event EventTakeDamage
  (params (amount :type Float%20%28single-precision%29) (attacker :type Actor%20Object%20Reference))
  (bind _output_get (Variables|Default|SetTowerHealth (- (Variables|Default|GetTowerHealth) amount)))
  (CallFunction|UpdateHealthBar)
  (if (<= _output_get 0.0)
    (bind _asbp_enemy_character (Utilities|Casting|CastToBP_EnemyCharacter attacker))
    (Variables|/Game/Blueprints/BP_EnemyCharacter.BP_EnemyCharacter_C|SetTargetToAttack _asbp_enemy_character 0)
    (Utilities|Time|SetTimerbyFunctionName 0 "Destroy" 1.0)
    (else
      (bind _asbp_enemy_character_2 (Utilities|Casting|CastToBP_EnemyCharacter attacker))
      (if (not (Utilities|Array|ContainsItem (Variables|Default|GetCurrentAttackers) _asbp_enemy_character_2))
        (Utilities|Array|Add (Variables|Default|GetCurrentAttackers) _asbp_enemy_character_2)))))

(fn ConstructionScript)

(fn Destroy
  (Actor|DestroyActor))

(fn UpdateHealthBar
  (CallFunction|UpdateHealthBox 0 (- (Variables|Default|GetMaxHealth) (Variables|Default|GetDamagedThreshold)) (- (Variables|Default|GetMaxHealth) (Variables|Default|GetDepletedThreshold)))
  (CallFunction|UpdateHealthBox 1 (- (Variables|Default|GetMaxHealth) (* (Variables|Default|GetDamagedThreshold) 2.0)) (- (Variables|Default|GetMaxHealth) (* (Variables|Default|GetDepletedThreshold) 2.0)))
  (CallFunction|UpdateHealthBox 2 (- (Variables|Default|GetMaxHealth) (* (Variables|Default|GetDamagedThreshold) 3.0)) 1e+01))

(fn UpdateHealthBox
  (params (BoxIndex :type Integer) (DamagedHealthThreshold :type Float%20%28single-precision%29) (DepletedHealthThreshold :type Float%20%28single-precision%29))
  (if (< (Variables|Default|GetTowerHealth) DamagedHealthThreshold)
    (bind _asbp_health_bar (Utilities|Casting|CastToBP_HealthBar (Variables|/Script/Engine.ChildActorComponent|GetChildActor (Variables|Default|GetHealthBar))))
    (Default|ChangeHealthBoxMaterial _asbp_health_bar BoxIndex "/Game/Materials/HealthBarDamaged_Inst.HealthBarDamaged_Inst")
    (if (< (Variables|Default|GetTowerHealth) DepletedHealthThreshold)
      (bind _asbp_health_bar_2 (Utilities|Casting|CastToBP_HealthBar (Variables|/Script/Engine.ChildActorComponent|GetChildActor (Variables|Default|GetHealthBar))))
      (Default|ChangeHealthBoxMaterial _asbp_health_bar_2 BoxIndex "/Game/Materials/HealthBarDepleted_Inst.HealthBarDepleted_Inst"))))