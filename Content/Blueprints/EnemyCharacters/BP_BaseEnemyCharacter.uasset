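; Base enemy character that moves to targets, attacks them and can ragdoll and stand back up.
; Its events drive AI movement and report state changes to BP_BaseEnemyController on arrival, target destruction and getting up.
; A looping timer damages the controller's current BP_MoveTarget until the associated attack target is destroyed.
; Falling enables mesh physics; getting up moves the actor to the mesh's XY, reattaches the mesh and disables physics.
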(event Custom|MoveToTarget
  (params (TargetToMoveTo :type Actor%20Object%20Reference) (AcceptanceRadius :type Float%20%28single-precision%29))
  (AI|AIMoveTo self "0, 0, 0" TargetToMoveTo AcceptanceRadius false
    (:OnSuccess
      (Default|SetState (Variables|Default|GetEnemyController) "NewEnumerator1"))))

(event Custom|Attack
  (bind _asbp_move_target (Utilities|Casting|CastToBP_MoveTarget (Variables|/Game/Blueprints/EnemyControllers/BP_BaseEnemyController.BP_BaseEnemyController_C|GetCurrentTarget (Variables|Default|GetEnemyController))))
  (Utilities|IsValid _asbp_move_target
    (:Is%20Valid
      (Default|TakeDamage _asbp_move_target (Variables|Default|GetDamage)))))

(event Custom|BeginAttack
  (params (MoveTarget :type BP%20Move%20Target%20Object%20Reference))
  (Utilities|IsValid MoveTarget
    (:Is%20Valid
      (Game|BindEventtoOnDestroyed (Variables|/Game/Blueprints/Environment/BP_MoveTarget.BP_MoveTarget_C|GetAssociatedAttackTarget MoveTarget) (delegate Custom|StopAttacking))
      (Utilities|Time|SetTimerbyFunctionName 0 "Attack" (Variables|Default|GetAttackFrequency) true))))

(event Custom|StopAttacking
  (params (DestroyedActor :type Actor%20Object%20Reference))
  (Utilities|Time|ClearTimerbyFunctionName 0 "Attack")
  (Default|SetState (Variables|Default|GetEnemyController) "NewEnumerator0"))

(event Custom|StartFalling
  (Physics|SetSimulatePhysics (Variables|Character|GetMesh) true))

(event Custom|GetUp
  (CallFunction|ResetCharacter)
  (Physics|SetSimulatePhysics (Variables|Character|GetMesh) false)
  (Default|SetState (Variables|Default|GetEnemyController) "NewEnumerator0"))

(event Custom|StopMoving
  (bind _enemycontroller (Variables|Default|GetEnemyController))
  (Utilities|IsValid _enemycontroller
    (:Is%20Valid
      (AI|Navigation|StopMovement _enemycontroller))))

(event EventBeginPlay
  (bind _asbp_base_enemy_controller (Utilities|Casting|CastToBP_BaseEnemyController (Pawn|GetController)))
  (Variables|Default|SetEnemyController _asbp_base_enemy_controller))

(fn ConstructionScript)

(fn GetStandUpLocation
  (bind _mesh (Variables|Character|GetMesh))
  (bind _returnvalue (Transformation|GetWorldLocation _mesh))
  (bind _output_get (LocalVariables|SetStandUpLocation (Math|Vector|MakeVector (.x _returnvalue) (.y _returnvalue) (Variables|/Script/Engine.CapsuleComponent|GetCapsuleHalfHeight (Variables|Collision|GetCapsuleComponent)))))
  (return _output_get))

(fn GetStandUpRotation
  (return (Math|Rotator|FindLookatRotation (Variables|/Script/Engine.SceneComponent|GetRelativeLocation (Variables|Character|GetMesh)) (Transformation|GetActorLocation (Variables|/Game/Blueprints/EnemyControllers/BP_BaseEnemyController.BP_BaseEnemyController_C|GetCurrentTarget (Variables|Default|GetEnemyController))))))

(fn ResetCharacter
  (Transformation|SetActorLocationAndRotation (CallFunction|GetStandUpLocation) "0, 0, 0")
  (Transformation|AttachComponentToComponent (Variables|Character|GetMesh) (Variables|Collision|GetCapsuleComponent) "None" "SnapToTarget" "SnapToTarget" "SnapToTarget" true)
  (Transformation|SetRelativeLocationAndRotation (Variables|Character|GetMesh) (Math|Vector|MakeVector 0.0 0.0 (* (Variables|/Script/Engine.CapsuleComponent|GetCapsuleHalfHeight (Variables|Collision|GetCapsuleComponent)) -1.0)) "0.000000,-90.000000,0.000000" false true))