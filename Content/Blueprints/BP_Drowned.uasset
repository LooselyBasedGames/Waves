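; BP_Drowned is an in-world counter that shows the number of enemies passed, presented as a "drowned" count.
; Every Tick it casts the game mode to BP_WavesGameMode, converts EnemiesPassed to text and writes it to its TextRender.
; The display polls rather than reacting to change events, and BeginPlay, overlap and construction add no logic of their own.
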(event EventBeginPlay
  (|CallParentFunction))

(event Collision|EventActorBeginOverlap
  (params (OtherActor :type Actor%20Object%20Reference)))

(event EventTick
  (params (DeltaSeconds :type Float%20%28single-precision%29))
  (bind _asbp_waves_game_mode (Utilities|Casting|CastToBP_WavesGameMode (Game|GetGameMode)))
  (bind _output_get (Variables|Default|SetDrownedText (Utilities|Text|ToText(Integer) (Variables|/Game/Blueprints/BP_WavesGameMode.BP_WavesGameMode_C|GetEnemiesPassed _asbp_waves_game_mode))))
  (Rendering|Components|TextRender|SetText (Variables|Default|GetTextRender) _output_get))

(fn ConstructionScript
  (|CallParentFunction))