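; BP_GravityGrenade is a grenade that can be picked up and spawns a BP_GravityForce actor where it detonates.
; A CookTime timer starts on BeginPlay and calls Detonate, which spawns the force actor and then destroys the grenade.
; Pickup and Drop extend the parent behavior: picking it up clears the timer, and dropping it restarts the full countdown.
; The mesh hit event is empty, so impacts do not trigger detonation.
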(event OnComponentHit(StaticMeshComponent)
  (params (HitComponent :type Primitive%20Component%20Object%20Reference) (OtherActor :type Actor%20Object%20Reference) (OtherComp :type Primitive%20Component%20Object%20Reference) (NormalImpulse :type Vector :default "0, 0, 0") (Hit :type Hit%20Result%20Structure%20%28by%20ref%29)))

(event EventBeginPlay
  (Utilities|Time|SetTimerbyFunctionName 0 "Detonate" (Variables|Default|GetCookTime)))

(event EventDrop
  (|CallParentFunction)
  (Utilities|Time|SetTimerbyFunctionName 0 "Detonate" (Variables|Default|GetCookTime)))

(event EventPickup
  (params (AttachTo :type Scene%20Component%20Object%20Reference))
  (|CallParentFunction AttachTo)
  (Utilities|Time|ClearTimerbyFunctionName 0 "Detonate"))

(fn ConstructionScript
  (|CallParentFunction))

(fn Detonate
  (Game|SpawnActorfromClass "/Game/Blueprints/BP_GravityForce.BP_GravityForce_C" (Transformation|GetActorTransform) "AlwaysSpawn" 0 0)
  (Actor|DestroyActor))